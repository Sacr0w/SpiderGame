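; Base Blueprint for weapon functions, giving weapons a shared player reference and damage formula.
; BeginPlay caches the first-person character in PlayerRef.
; DamageCalc multiplies weapon damage by a base percent and the player's base damage percent, then divides by 100, re-casting the player rather than using PlayerRef.
; Unequip, OnUpgrade, ConvertToPickup and OverallDamageCalc are empty here, apparently left as hooks for child weapons.
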(event Custom|Unequip
  (params (SpawnPickup :type Boolean)))

(event Custom|OnUpgrade
  (params (Upgrade%20#1 :type Boolean)))

(event EventBeginPlay
  (bind _asbp_first_person_character (Utilities|Casting|CastToBP_FirstPersonCharacter (Game|GetPlayerCharacter 0)))
  (Variables|Default|SetPlayerRef _asbp_first_person_character))

(event EventTick
  (params (DeltaSeconds :type Float%20%28single-precision%29)))

(fn ConverttoPickup)

(fn DamageCalc
  (params (WeaponDamage :type Float%20%28double-precision%29) (BasePercent :type Float%20%28double-precision%29))
  (bind _output_get (LocalVariables|SetDamageCalculation WeaponDamage))
  (bind _output_get_2 (LocalVariables|SetDamageCalculation (* _output_get BasePercent)))
  (bind _asbp_first_person_character (Utilities|Casting|CastToBP_FirstPersonCharacter (Game|GetPlayerCharacter 0)))
  (return (/ (* _output_get_2 (Variables|/Game/NatsBlueprints/Blueprints/Player/BP_FirstPersonCharacter.BP_FirstPersonCharacter_C|GetPlayerBaseDamagePercent _asbp_first_person_character)) 1e+02)))