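; Base weapon pickup actor that shows an info widget when highlighted and destroys itself after an idle timeout unless stored.
; Pickup records the stored state, and both pickup and highlight restart the despawn timer through a retriggerable delay.
; Repeated highlight calls hold a short-lived flag that Tick uses to toggle widget visibility.
; InitialiseInfo fills the widget from a data table row, with an optional damage override.
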(event Custom|Pickup
  (params (PlayerRef :type BP%20First%20Person%20Character%20Object%20Reference) (LeftHanded :type Boolean) (Storing :type Boolean) (PickupFromStorage :type Boolean))
  (Variables|Default|Setstored? Storing)
  (Rendering|SetVisibility (Variables|Default|GetWeaponInfo) false false)
  (Utilities|FlowControl|RetriggerableDelay 3e+01)
  (if (not (Variables|Default|Getstored?))
    (Actor|DestroyActor)))

(event Custom|Highlight
  (Utilities|FlowControl|Sequence
    (:then_0
      (Utilities|FlowControl|RetriggerableDelay 3e+01)
      (if (not (Variables|Default|Getstored?))
        (Actor|DestroyActor)))
    (:then_1
      (Variables|Default|SetHighlighted true)
      (Utilities|FlowControl|RetriggerableDelay 0.05)
      (Variables|Default|SetHighlighted false))))

(event EventBeginPlay
  (Rendering|SetVisibility (Variables|Default|GetWeaponInfo) false false)
  (Utilities|FlowControl|RetriggerableDelay 3e+01)
  (if (not (Variables|Default|Getstored?))
    (Actor|DestroyActor)))

(event Collision|EventActorBeginOverlap
  (params (OtherActor :type Actor%20Object%20Reference)))

(event EventTick
  (params (DeltaSeconds :type Float%20%28single-precision%29))
  (bind _weaponinfo (Variables|Default|GetWeaponInfo))
  (if (Variables|Default|GetHighlighted)
    (Rendering|SetVisibility _weaponinfo true false)
    (else
      (Rendering|SetVisibility _weaponinfo false false))))

(fn ConstructionScript)

(fn InitialiseInfo
  (params (DamageOverride :type Float%20%28double-precision%29))
  (bind _aswb_weapon_info (Utilities|Casting|CastToWB_WeaponInfo (UserInterface|GetUserWidgetObject (Variables|Default|GetWeaponInfo))))
  (LocalVariables|SetWeaponInfoRef _aswb_weapon_info)
  (bind _returnvalue (Class|DataTableFunctionLibrary|DoesDataTableRowExist "/Game/NatsBlueprints/Blueprints/Weapons/WeaponInfoTable.WeaponInfoTable" (Variables|Default|GetInfoRow)))
  (if _returnvalue
    (bind _returnvalue_2 (Utilities|GetDataTableRow "/Game/NatsBlueprints/Blueprints/Weapons/WeaponInfoTable.WeaponInfoTable" (Variables|Default|GetInfoRow))
      (:then
        (LocalVariables|SetRowRef _returnvalue_2)
        (Utilities|FlowControl|Sequence
          (:then_0
            (Variables|/Game/NatsBlueprints/Blueprints/Weapons/WB_WeaponInfo.WB_WeaponInfo_C|SetName (LocalVariables|GetWeaponInfoRef) (.Name (Utilities|Struct|BreakWeaponInfoStruct (LocalVariables|GetRowRef)))))
          (:then_1
            (Variables|/Game/NatsBlueprints/Blueprints/Weapons/WB_WeaponInfo.WB_WeaponInfo_C|SetFlavourText (LocalVariables|GetWeaponInfoRef) (.FlavourText (Utilities|Struct|BreakWeaponInfoStruct (LocalVariables|GetRowRef)))))
          (:then_2
            (Variables|/Game/NatsBlueprints/Blueprints/Weapons/WB_WeaponInfo.WB_WeaponInfo_C|SetDescriptionPart1 (LocalVariables|GetWeaponInfoRef) (.DescriptionPart1 (Utilities|Struct|BreakWeaponInfoStruct (LocalVariables|GetRowRef)))))
          (:then_3
            (Variables|/Game/NatsBlueprints/Blueprints/Weapons/WB_WeaponInfo.WB_WeaponInfo_C|SetDamage (LocalVariables|GetWeaponInfoRef) (Math|Integer|SelectInt (.Damage (Utilities|Struct|BreakWeaponInfoStruct (LocalVariables|GetRowRef))) (Math|Float|Truncate DamageOverride) (== DamageOverride 0.0))))
          (:then_4
            (Variables|/Game/NatsBlueprints/Blueprints/Weapons/WB_WeaponInfo.WB_WeaponInfo_C|SetDescriptionPart2 (LocalVariables|GetWeaponInfoRef) (.DescriptionPart2 (Utilities|Struct|BreakWeaponInfoStruct (LocalVariables|GetRowRef)))))
          (:then_5
            (Variables|/Game/NatsBlueprints/Blueprints/Weapons/WB_WeaponInfo.WB_WeaponInfo_C|SetmodifiedDamage? (LocalVariables|GetWeaponInfoRef) (.modifiedDamage? (Utilities|Struct|BreakWeaponInfoStruct (LocalVariables|GetRowRef)))))
          (:then_6
            (Variables|/Game/NatsBlueprints/Blueprints/Weapons/WB_WeaponInfo.WB_WeaponInfo_C|SetTwoHanded (LocalVariables|GetWeaponInfoRef) (.Two-Handed? (Utilities|Struct|BreakWeaponInfoStruct (LocalVariables|GetRowRef)))))
          (:then_7
            (Variables|/Game/NatsBlueprints/Blueprints/Weapons/WB_WeaponInfo.WB_WeaponInfo_C|SetCost (LocalVariables|GetWeaponInfoRef) (.Cost (Utilities|Struct|BreakWeaponInfoStruct (LocalVariables|GetRowRef))))))))))