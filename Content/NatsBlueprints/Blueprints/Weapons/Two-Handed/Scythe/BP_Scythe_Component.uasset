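; Two-handed scythe weapon component that attaches to the first-person character, occupies both hands and adds its input mapping context.
; Left click plays a montage whose notify sphere-overlaps ahead of the camera, damaging Animal_Parent pawns through DamageCalc and drawing a debug sphere.
; The block input triggers Empower on the player at the cost of current health.
; Unequip can throw a pickup carrying both upgrade counts, then removes the mapping and component.
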(event Input|EnhancedActionEvents|EnhancedInputActionIA_LeftClick
  (params (ActionValue :type Boolean) (ElapsedSeconds :type Float%20%28double-precision%29) (TriggeredSeconds :type Float%20%28double-precision%29) (InputAction :type Input%20Action%20Object%20Reference :default "/Game/NatsBlueprints/Input/Actions/IA_LeftClick.IA_LeftClick"))
  (bind _first_personcharacter (Variables|Default|GetFirst%20PersonCharacter))
  (bind _first_personcharacter_2 (Variables|Default|GetFirst%20PersonCharacter))
  (bind _firstpersoncamera (Variables|/Game/NatsBlueprints/Blueprints/Player/BP_FirstPersonCharacter.BP_FirstPersonCharacter_C|GetFirstPersonCamera _first_personcharacter_2))
  (bind _returnvalue (Transformation|GetWorldRotation _firstpersoncamera))
  (bind _returnvalue_2 (Transformation|GetWorldLocation _firstpersoncamera))
  (bind _returnvalue_3 (Math|Vector|GetForwardVector _returnvalue))
  (bind _returnvalue_4 (* _returnvalue_3 1.2e+02))
  (bind _returnvalue_5 (+ _returnvalue_2 _returnvalue_4))
  ;[1 1 1] Attack Logic
  (:Triggered
    (if (not (Variables|Default|GetisEmpowering))
      (if (not (Variables|Default|GetIsAttacking))
        (if (not (Variables|/Game/NatsBlueprints/Blueprints/Player/BP_FirstPersonCharacter.BP_FirstPersonCharacter_C|GetisAttacking%28Player%29 _first_personcharacter))
          (if (not (Variables|/Game/NatsBlueprints/Blueprints/Player/BP_FirstPersonCharacter.BP_FirstPersonCharacter_C|GetisKicking _first_personcharacter))
            (Variables|Default|SetIsAttacking true)
            (Variables|/Game/NatsBlueprints/Blueprints/Player/BP_FirstPersonCharacter.BP_FirstPersonCharacter_C|SetisAttacking%28Player%29 (Variables|Default|GetFirst%20PersonCharacter) true)
            (bind _notifyname (Animation|Montage|PlayMontage (Variables|/Game/NatsBlueprints/Blueprints/Player/BP_FirstPersonCharacter.BP_FirstPersonCharacter_C|GetFirstPersonMesh (Variables|Default|GetFirst%20PersonCharacter)) "/Game/untitled_category/ShovelAttackMontage.ShovelAttackMontage" 0.6)
              (:OnNotifyBegin
                (if (or (== _notifyname "IMPACT") (== "" "Impact"))
                  (bind _outactors (Actor|GetAllActorsOfClass "/Game/NatsBlueprints/Blueprints/Player/BP_FirstPersonCharacter.BP_FirstPersonCharacter_C"))
                  (bind (_outactors_2 _returnvalue_6) (Collision|SphereOverlapActors _returnvalue_5 1.3e+02 (Utilities|Array|MakeArray "ObjectTypeQuery3") "/Game/Assets/Animals/Animal_Parent.Animal_Parent_C" _outactors))
                  (Rendering|Debug|DrawDebugSphere _returnvalue_5 1.3e+02 12 "(R=1.000000,G=1.000000,B=1.000000,A=1.000000)" 5.0 1.0)
                  (if _returnvalue_6
                    (Audio|PlaySoundatLocation "/Game/Assets/Audio/Shovel_Hit_01.Shovel_Hit_01" "0, 0, 0" "0, 0, 0" 1.0 1.0 0.0 0 0 0 0)
                    (else
                      (Audio|PlaySoundatLocation "/Game/Assets/Audio/Shovel_Miss.Shovel_Miss" "0, 0, 0" "0, 0, 0" 1.0 1.0 0.0 0 0 0 0)))
                  (for _array_element _outactors_2
                    (bind _asanimal_parent (Utilities|Casting|CastToAnimal_Parent _array_element))
                    (bind _finaldamage (CallFunction|DamageCalc (Variables|Default|GetDamage) (Variables|Default|GetBasePercent)))
                    (Development|PrintString (Utilities|String|ToString(Float) _finaldamage))
                    (Default|OnHit _asanimal_parent _finaldamage)
                    (Utilities|FlowControl|DelayUntilNextTick))
                  (else
                    (Variables|Default|SetIsAttacking false)
                    (Variables|/Game/NatsBlueprints/Blueprints/Player/BP_FirstPersonCharacter.BP_FirstPersonCharacter_C|SetisAttacking%28Player%29 (Variables|Default|GetFirst%20PersonCharacter) false)))))))))))

(event Input|EnhancedActionEvents|EnhancedInputActionIA_Shovel_Block
  (params (ActionValue :type Boolean) (ElapsedSeconds :type Float%20%28double-precision%29) (TriggeredSeconds :type Float%20%28double-precision%29) (InputAction :type Input%20Action%20Object%20Reference :default "/Game/NatsBlueprints/Input/Actions/IA_Shovel_Block.IA_Shovel_Block"))
  (bind _first_personcharacter (Variables|Default|GetFirst%20PersonCharacter))
  ;[1 1 1] ScytheEmpowerLogic
  (:Triggered
    (if (not (Variables|/Game/NatsBlueprints/Blueprints/Player/BP_FirstPersonCharacter.BP_FirstPersonCharacter_C|GetisEmpowered? _first_personcharacter))
      (Variables|Default|SetisEmpowering true)
      (Variables|/Game/NatsBlueprints/Blueprints/Player/BP_FirstPersonCharacter.BP_FirstPersonCharacter_C|SetisAttacking%28Player%29 _first_personcharacter true)
      (bind _notifyname (Animation|Montage|PlayMontage (Variables|/Game/NatsBlueprints/Blueprints/Player/BP_FirstPersonCharacter.BP_FirstPersonCharacter_C|GetFirstPersonMesh (Variables|Default|GetFirst%20PersonCharacter)) "/Game/Imports/Viewmodel_Testing/FPV_Limbs/SpraycanLighter_Anims/Lighter_Equip_Montage.Lighter_Equip_Montage" 0.8)
        (:OnCompleted
          (Variables|Default|SetisEmpowering false)
          (Variables|/Game/NatsBlueprints/Blueprints/Player/BP_FirstPersonCharacter.BP_FirstPersonCharacter_C|SetisAttacking%28Player%29 _first_personcharacter false))
        (:OnNotifyBegin
          (if (== _notifyname "Activate")
            (Default|Empower _first_personcharacter)
            (Default|OnHit _first_personcharacter 0.25 true)))))))

(event EventBeginPlay
  ;[1 1 1] EquipLogic
  (|CallParentFunction)
  (bind _asbp_first_person_character (Utilities|Casting|CastToBP_FirstPersonCharacter (Components|GetOwner)))
  (bind _output_get (Variables|Default|SetFirst%20PersonCharacter _asbp_first_person_character))
  (Transformation|AttachComponentToComponent (Variables|/Game/NatsBlueprints/Blueprints/Player/BP_FirstPersonCharacter.BP_FirstPersonCharacter_C|GetFirstPersonMesh _output_get) "TwoHandedShovelPoint" "SnapToTarget" "SnapToTarget" "SnapToTarget" true)
  (Variables|/Game/NatsBlueprints/Blueprints/Player/BP_FirstPersonCharacter.BP_FirstPersonCharacter_C|SetbhasScythe? (Variables|Default|GetFirst%20PersonCharacter) true)
  (Variables|/Game/NatsBlueprints/Blueprints/Player/BP_FirstPersonCharacter.BP_FirstPersonCharacter_C|SetleftHandAvailable (Variables|Default|GetFirst%20PersonCharacter) false)
  (Variables|/Game/NatsBlueprints/Blueprints/Player/BP_FirstPersonCharacter.BP_FirstPersonCharacter_C|SetrightHandAvailable (Variables|Default|GetFirst%20PersonCharacter) false)
  (Variables|/Game/NatsBlueprints/Blueprints/Player/BP_FirstPersonCharacter.BP_FirstPersonCharacter_C|SetisCurrentWeaponTwoHanded? (Variables|Default|GetFirst%20PersonCharacter) true)
  (bind _asplayer_controller (Utilities|Casting|CastToPlayerController (Pawn|GetController (Variables|Default|GetFirst%20PersonCharacter))))
  (Utilities|IsValid (PlayerController|LocalPlayerSubsystems|GetEnhancedInputLocalPlayerSubsystem _asplayer_controller)
    (:Is%20Valid
      (Input|AddMappingContext (PlayerController|LocalPlayerSubsystems|GetEnhancedInputLocalPlayerSubsystem _asplayer_controller) "/Game/NatsBlueprints/Input/IMC_Scythe.IMC_Scythe" 1 "(bIgnoreAllPressedKeysUntilRelease=True,bForceImmediately=False)"))))

(event EventUnequip
  (params (SpawnPickup :type Boolean))
  (bind _first_personcharacter (Variables|Default|GetFirst%20PersonCharacter))
  (bind _first_personcharacter_2 (Variables|Default|GetFirst%20PersonCharacter))
  ;[1 1 1] Unequip Logic
  (if SpawnPickup
    (bind _returnvalue (Game|SpawnActorfromClass "/Game/NatsBlueprints/Blueprints/Weapons/Two-Handed/Scythe/BP_Pickup_Scythe.BP_Pickup_Scythe_C" (Transformation|GetActorTransform _first_personcharacter) "Undefined" "MultiplyWithRoot" 0 0))
    (Physics|AddForce (Variables|/Game/NatsBlueprints/Blueprints/Weapons/Two-Handed/Scythe/BP_Pickup_Scythe.BP_Pickup_Scythe_C|GetSkeletalMesh _returnvalue) (+ (Transformation|GetWorldLocation) (* (Math|Vector|GetForwardVector (Transformation|GetWorldRotation (Variables|/Game/NatsBlueprints/Blueprints/Player/BP_FirstPersonCharacter.BP_FirstPersonCharacter_C|GetFirstPersonCamera (Variables|Default|GetFirst%20PersonCharacter)))) 2.5e+04)) "None" true)
    (Variables|/Game/NatsBlueprints/Blueprints/Weapons/BP_WeaponPickup_Parent.BP_WeaponPickup_Parent_C|SetupgradeAmount%28A%29 _returnvalue (Variables|Default|GetupgradeAmount%281%29))
    (Variables|/Game/NatsBlueprints/Blueprints/Weapons/BP_WeaponPickup_Parent.BP_WeaponPickup_Parent_C|SetupgradeAmount%28B%29 _returnvalue (Variables|Default|GetupgradeAmount%282%29)))
  (Variables|/Game/NatsBlueprints/Blueprints/Player/BP_FirstPersonCharacter.BP_FirstPersonCharacter_C|SetbhasScythe? _first_personcharacter_2 false)
  (Variables|/Game/NatsBlueprints/Blueprints/Player/BP_FirstPersonCharacter.BP_FirstPersonCharacter_C|SetisCurrentWeaponTwoHanded? _first_personcharacter_2 false)
  (bind _asplayer_controller (Utilities|Casting|CastToPlayerController (Pawn|GetController _first_personcharacter))
    (:then
      (Utilities|IsValid (PlayerController|LocalPlayerSubsystems|GetEnhancedInputLocalPlayerSubsystem _asplayer_controller)
        (:Is%20Valid
          (Input|RemoveMappingContext (PlayerController|LocalPlayerSubsystems|GetEnhancedInputLocalPlayerSubsystem _asplayer_controller) "/Game/NatsBlueprints/Input/IMC_Scythe.IMC_Scythe" "(bIgnoreAllPressedKeysUntilRelease=True,bForceImmediately=False)"))
        (:Is%20Not%20Valid
          _)))
    (:CastFailed
      _))
  (Components|DestroyComponent))

(event EventOnUpgrade
  (params (Upgrade%20#1 :type Boolean))
  (if Upgrade%20#1
    (Variables|Default|SetupgradeAmount%281%29 (+ (Variables|Default|GetupgradeAmount%281%29) 1))
    (else
      (Variables|Default|SetupgradeAmount%282%29 (+ (Variables|Default|GetupgradeAmount%282%29) 1)))))

(event EventTick
  (params (DeltaSeconds :type Float%20%28single-precision%29))
  (|CallParentFunction DeltaSeconds)
  (if (not (> (Variables|Default|GetupgradeAmount%281%29) 0))
    (if (> (Variables|Default|GetupgradeAmount%282%29) 0)
      _)))