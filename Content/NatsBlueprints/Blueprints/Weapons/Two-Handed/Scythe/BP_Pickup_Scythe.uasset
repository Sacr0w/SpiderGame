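; Scythe weapon pickup that either stores itself or equips the scythe as the player's two-handed weapon, extending a parent pickup class.
; Storing tags, hides and disables collision on the actor; equipping adds a scythe component to the player, copies both upgrade amounts and destroys the pickup.
; Tick swaps the mesh material for highlighting and keeps the weapon info display offset from the mesh, turned toward the player's view.
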(event EventBeginPlay
  (|CallParentFunction)
  (Variables|Default|SetMeshToUse (Variables|Default|GetSkeletalMesh))
  (CallFunction|InitialiseInfo 0.0))

(event EventPickup
  (params (PlayerRef :type BP%20First%20Person%20Character%20Object%20Reference) (LeftHanded :type Boolean) (Storing :type Boolean) (PickupFromStorage :type Boolean))
  ;[0.05 0.05 0.05] Pickup Logic
  (|CallParentFunction PlayerRef LeftHanded Storing PickupFromStorage)
  (if (not (and (Actor|ActorHasTag self "Stored") (not PickupFromStorage)))
    (if Storing
      (Variables|Default|SetTags (Utilities|Array|MakeArray "Stored"))
      (Rendering|SetActorHiddenInGame true)
      (Collision|SetActorEnableCollision false)
      (else
        (bind _output_get (Variables|Default|SetFirstPersonCharacterReference PlayerRef))
        (bind _returnvalue (AddComponent|AddBPScytheComponent _output_get false))
        (Variables|/Game/NatsBlueprints/Blueprints/Weapons/BP_WeaponFunction_Parent.BP_WeaponFunction_Parent_C|SetupgradeAmount%281%29 _returnvalue (Variables|Default|GetupgradeAmount%28A%29))
        (Variables|/Game/NatsBlueprints/Blueprints/Weapons/BP_WeaponFunction_Parent.BP_WeaponFunction_Parent_C|SetupgradeAmount%282%29 _returnvalue (Variables|Default|GetupgradeAmount%28B%29))
        (Variables|/Game/NatsBlueprints/Blueprints/Player/BP_FirstPersonCharacter.BP_FirstPersonCharacter_C|SettwoHandedWeaponEquipped _output_get _returnvalue)
        (Actor|DestroyActor)))))

(event EventTick
  (params (DeltaSeconds :type Float%20%28single-precision%29))
  (bind _meshtouse (Variables|Default|GetMeshToUse))
  ;[0.03646 0.03646 0.03646] Highlight Logic
  (|CallParentFunction 0.0)
  (if (Variables|Default|GetHighlighted)
    (Rendering|Material|SetMaterial _meshtouse 0 "/Game/LevelPrototyping/Materials/MI_Solid_Blue.MI_Solid_Blue")
    (else
      (Rendering|Material|SetMaterial _meshtouse 0 "/Game/Assets/Animals/Bee_V2/Bee.Bee")))
  (Transformation|SetWorldLocationAndRotation (Variables|Default|GetWeaponInfo) (+ (Transformation|GetWorldLocation (Variables|Default|GetSkeletalMesh)) (Variables|Default|GetInfoScreenOffset)) (Math|Rotator|FindLookatRotation (Transformation|GetWorldLocation (Variables|Default|GetWeaponInfo)) (.OutLocation (Actor|GetActorEyesViewPoint (Game|GetPlayerCharacter 0)))) false true))

(fn ConstructionScript)