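; Pickup actor for the two-handed spraycan-and-lighter flamethrower, with a highlight material and an info display that follows the mesh and faces the player.
; Storing it tags the actor as Stored, then hides it and disables collision.
; Equipping adds a flamethrower component to the player character, copies both upgrade amounts onto it, sets it as the two-handed weapon, plays a sound and destroys the pickup.
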(event EventBeginPlay
  (|CallParentFunction)
  (CallFunction|InitialiseInfo 0.0))

(event EventPickup
  (params (PlayerRef :type BP%20First%20Person%20Character%20Object%20Reference) (LeftHanded :type Boolean) (Storing :type Boolean) (PickupFromStorage :type Boolean))
  (|CallParentFunction PlayerRef LeftHanded Storing PickupFromStorage)
  (if (not (and (Actor|ActorHasTag "Stored") (not PickupFromStorage)))
    (if Storing
      (Variables|Default|SetTags (Utilities|Array|MakeArray "Stored"))
      (Rendering|SetActorHiddenInGame true)
      (Collision|SetActorEnableCollision false)
      (else
        (bind _output_get (Variables|Default|SetFirstPersonCharacterRef PlayerRef))
        (bind _returnvalue (AddComponent|AddBPFlamethrowerComponent _output_get false))
        (Variables|/Game/NatsBlueprints/Blueprints/Weapons/Two-Handed/Spraycan_Lighter/BP_Flamethrower_Component.BP_Flamethrower_Component_C|SetSkeletalMeshRef _returnvalue _returnvalue)
        (Variables|/Game/NatsBlueprints/Blueprints/Weapons/BP_WeaponFunction_Parent.BP_WeaponFunction_Parent_C|SetupgradeAmount%281%29 _returnvalue (Variables|Default|GetupgradeAmount%28A%29))
        (Variables|/Game/NatsBlueprints/Blueprints/Weapons/BP_WeaponFunction_Parent.BP_WeaponFunction_Parent_C|SetupgradeAmount%282%29 _returnvalue (Variables|Default|GetupgradeAmount%28B%29))
        (Variables|/Game/NatsBlueprints/Blueprints/Player/BP_FirstPersonCharacter.BP_FirstPersonCharacter_C|SettwoHandedWeaponEquipped _output_get _returnvalue)
        (Audio|PlaySound2D "/Game/NatsBlueprints/Blueprints/Weapons/One-Handed/Spraycan/SpraycanEquip.SpraycanEquip" 1.0 1.0 0.0 0 0)
        (Actor|DestroyActor)))))

(event EventTick
  (params (DeltaSeconds :type Float%20%28single-precision%29))
  (bind _skeletalmesh (Variables|Default|GetSkeletalMesh))
  (|CallParentFunction 0.0)
  (if (Variables|Default|GetHighlighted)
    (Rendering|Material|SetMaterial _skeletalmesh 0 "/Game/LevelPrototyping/Materials/MI_Solid_Blue.MI_Solid_Blue")
    (else
      (Rendering|Material|SetMaterial _skeletalmesh 0 "/Game/Imports/Viewmodel_Testing/FPV_Spraycan/M_SpraycanFire.M_SpraycanFire")
      (Rendering|Material|SetMaterial _skeletalmesh 1 "/Game/Imports/Viewmodel_Testing/FPV_Spraycan/Outline.Outline")))
  (Transformation|SetWorldLocationAndRotation (Variables|Default|GetWeaponInfo) (+ (Transformation|GetWorldLocation (Variables|Default|GetSkeletalMesh)) (Variables|Default|GetInfoScreenOffset)) (Math|Rotator|FindLookatRotation (Transformation|GetWorldLocation (Variables|Default|GetWeaponInfo)) (.OutLocation (Actor|GetActorEyesViewPoint (Game|GetPlayerCharacter 0)))) false true))

(event Collision|EventActorBeginOverlap
  (params (OtherActor :type Actor%20Object%20Reference))
  (|CallParentFunction OtherActor) ; This node is disabled and will not be called.\nDrag off pins to build functionality.
)

(fn ConstructionScript
  (|CallParentFunction))