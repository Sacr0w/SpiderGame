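; Two-handed spraycan-and-lighter weapon component that gives the first-person character a toggleable flamethrower.
; BeginPlay attaches can and lighter to the hands, marks both occupied and adds its input mapping context.
; Spraying spawns an attached flame or plain-spray damage hitbox with matching looped animation and sound, based on lighter state.
; Tick drains ammo while attacking and recharges it after a delay; Unequip cleans up, optionally throwing a pickup.
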(event Input|EnhancedActionEvents|EnhancedInputActionIA_ToggleLighter
  (params (ActionValue :type Boolean) (ElapsedSeconds :type Float%20%28double-precision%29) (TriggeredSeconds :type Float%20%28double-precision%29) (InputAction :type Input%20Action%20Object%20Reference :default "/Game/NatsBlueprints/Input/Actions/IA_ToggleLighter.IA_ToggleLighter"))
  (bind _first_personcharacter (Variables|Default|GetFirst%20PersonCharacter))
  (:Triggered
    (if (not (Variables|Default|GetIsAttacking))
      (if (Variables|Default|GetlighterActive?)
        (Variables|Default|SetisToggling true)
        (Variables|Default|SetlighterActive? false)
        (Variables|/Game/NatsBlueprints/Blueprints/Player/BP_FirstPersonCharacter.BP_FirstPersonCharacter_C|SetbLighterActive _first_personcharacter false)
        (Utilities|FlowControl|Delay 0.5)
        (else
          (Variables|Default|SetisToggling true)
          (Variables|Default|SetlighterActive? true)
          (Variables|/Game/NatsBlueprints/Blueprints/Player/BP_FirstPersonCharacter.BP_FirstPersonCharacter_C|SetbLighterActive _first_personcharacter true)
          (Utilities|FlowControl|Delay 0.5)))
      (Variables|Default|SetisToggling false))))

(event Input|EnhancedActionEvents|EnhancedInputActionIA_SprayLeft
  (params (ActionValue :type Boolean) (ElapsedSeconds :type Float%20%28double-precision%29) (TriggeredSeconds :type Float%20%28double-precision%29) (InputAction :type Input%20Action%20Object%20Reference :default "/Game/NatsBlueprints/Input/Actions/IA_SprayLeft.IA_SprayLeft"))
  (bind _first_personcharacter (Variables|Default|GetFirst%20PersonCharacter))
  (bind _skeletalmeshref (Variables|Default|GetSkeletalMeshRef))
  (bind _first_personcharacter_2 (Variables|Default|GetFirst%20PersonCharacter))
  ;[1 0.01042 0.01042] Attack Logic (Left)
  ;;[1 1 1] Attack Start
  (:Triggered
    (if (> (Variables|Default|GetammoAmount) 1e+01)
      (if (not (Variables|Default|GetisToggling))
        (if (not (Variables|Default|GetIsAttacking))
          (if (not (Variables|Default|GetisDisabling))
            (Variables|/Game/NatsBlueprints/Blueprints/Player/BP_FirstPersonCharacter.BP_FirstPersonCharacter_C|SetisAttacking%28Player%29 _first_personcharacter true)
            (Variables|/Game/NatsBlueprints/Blueprints/Player/BP_FirstPersonCharacter.BP_FirstPersonCharacter_C|SetbFlamethrowerAttacking _first_personcharacter true)
            (Variables|Default|SetIsAttacking true)
            (Components|Animation|PlayAnimation _skeletalmeshref "/Game/Imports/Viewmodel_Testing/FPV_Spraycan/Spraycan_AttackStart.Spraycan_AttackStart" false)
            (Utilities|FlowControl|Delay 0.05)
            (Components|Animation|PlayAnimation _skeletalmeshref "/Game/Imports/Viewmodel_Testing/FPV_Spraycan/Spraycan_AttackLoop.Spraycan_AttackLoop" true)
            (bind _returnvalue (Game|SpawnActorfromClass (select (Variables|Default|GetlighterActive?) "/Game/NatsBlueprints/Blueprints/Weapons/Two-Handed/Spraycan_Lighter/FlamethrowerParticleHitbox.FlamethrowerParticleHitbox_C" "/Game/NatsBlueprints/Blueprints/Weapons/One-Handed/Spraycan/SpraycanParticleHitbox.SpraycanParticleHitbox_C") (Transformation|GetWorldTransform) "Undefined" "MultiplyWithRoot" 0 0))
            (Transformation|AttachComponentToComponent _returnvalue self "CapSocket" "SnapToTarget" "SnapToTarget" "SnapToTarget" true)
            (bind _finaldamage (CallFunction|DamageCalc (Variables|Default|GetbaseDamage) (Variables|Default|GetWeaponBaseDamagePercent)))
            (Variables|/Game/NatsBlueprints/Blueprints/Weapons/One-Handed/Spraycan/SpraycanHitboxParent.SpraycanHitboxParent_C|SetDamage _returnvalue _finaldamage)
            (bind _returnvalue_2 (Audio|CreateSound2D (select (Variables|Default|GetlighterActive?) "/Game/NatsBlueprints/Blueprints/Weapons/Two-Handed/Spraycan_Lighter/Flamethrower_Attack.Flamethrower_Attack" "/Game/NatsBlueprints/Blueprints/Weapons/One-Handed/Spraycan/Spraycan_Attack.Spraycan_Attack") 1.0 1.0 0.0 0))
            (Audio|Components|Audio|Play _returnvalue_2 0.0))))))
  (:Canceled
    ;;[1 1 1] Attack End
    (if (Variables|Default|GetIsAttacking) :!label _label
      (if (not (Variables|Default|GetisToggling))
        (if (not (Variables|Default|GetisDisabling))
          (Variables|Default|SetisDisabling true)
          (Variables|/Game/NatsBlueprints/Blueprints/Player/BP_FirstPersonCharacter.BP_FirstPersonCharacter_C|SetisAttacking%28Player%29 _first_personcharacter_2 false)
          (Variables|/Game/NatsBlueprints/Blueprints/Player/BP_FirstPersonCharacter.BP_FirstPersonCharacter_C|SetbFlamethrowerAttacking _first_personcharacter_2 false)
          (Variables|Default|SetIsAttacking false)
          (Components|Animation|PlayAnimation _skeletalmeshref "/Game/Imports/Viewmodel_Testing/FPV_Spraycan/Spraycan_AttackEnd.Spraycan_AttackEnd" false)
          (Utilities|FlowControl|Delay 0.05)
          (Utilities|IsValid _returnvalue
            (:Is%20Valid
              (Variables|/Game/NatsBlueprints/Blueprints/Weapons/One-Handed/Spraycan/SpraycanHitboxParent.SpraycanHitboxParent_C|Setactive _returnvalue false))
            (:Is%20Not%20Valid
              _))
          (Utilities|FlowControl|Delay 0.05)
          (Components|Animation|PlayAnimation _skeletalmeshref "/Game/Imports/Viewmodel_Testing/FPV_Spraycan/Spraycan_CapIdle.Spraycan_CapIdle" true)
          (Variables|Default|SetisDisabling false)
          (Utilities|IsValid _returnvalue_2
            (:Is%20Valid
              (Audio|Components|Audio|Stop _returnvalue_2)
              (Components|DestroyComponent _returnvalue_2)))))))
  (:Completed
    (goto _label)))

(event EventBeginPlay
  ;[1 1 1] Equip Logic
  (|CallParentFunction)
  (bind _asbp_first_person_character (Utilities|Casting|CastToBP_FirstPersonCharacter (Components|GetOwner)))
  (bind _output_get (Variables|Default|SetFirst%20PersonCharacter _asbp_first_person_character))
  (Variables|/Game/NatsBlueprints/Blueprints/Player/BP_FirstPersonCharacter.BP_FirstPersonCharacter_C|SetbLighterActive (Variables|Default|GetFirst%20PersonCharacter) true)
  (bind _returnvalue (Game|SpawnActorfromClass "/Game/NatsBlueprints/Blueprints/Weapons/Two-Handed/Spraycan_Lighter/BP_Lighter.BP_Lighter_C" (Math|Transform|MakeTransform "0, 0, 0") "Undefined" "MultiplyWithRoot" 0 0))
  (Transformation|AttachComponentToComponent _returnvalue (Variables|/Game/NatsBlueprints/Blueprints/Player/BP_FirstPersonCharacter.BP_FirstPersonCharacter_C|GetFirstPersonMesh _output_get) "LeftHandedLighterPoint" "KeepRelative" "KeepRelative" "KeepRelative" true)
  (Transformation|AttachComponentToComponent (Variables|/Game/NatsBlueprints/Blueprints/Player/BP_FirstPersonCharacter.BP_FirstPersonCharacter_C|GetFirstPersonMesh _output_get) "RightHandedSpraycanPoint" "SnapToTarget" "SnapToTarget" "SnapToTarget" true)
  (Variables|/Game/NatsBlueprints/Blueprints/Player/BP_FirstPersonCharacter.BP_FirstPersonCharacter_C|SetbHasFlamethrower (Variables|Default|GetFirst%20PersonCharacter) true)
  (Variables|/Game/NatsBlueprints/Blueprints/Player/BP_FirstPersonCharacter.BP_FirstPersonCharacter_C|SetleftHandAvailable (Variables|Default|GetFirst%20PersonCharacter) false)
  (Variables|/Game/NatsBlueprints/Blueprints/Player/BP_FirstPersonCharacter.BP_FirstPersonCharacter_C|SetrightHandAvailable (Variables|Default|GetFirst%20PersonCharacter) false)
  (Variables|/Game/NatsBlueprints/Blueprints/Player/BP_FirstPersonCharacter.BP_FirstPersonCharacter_C|SetisCurrentWeaponTwoHanded? (Variables|Default|GetFirst%20PersonCharacter) true)
  (bind _asplayer_controller (Utilities|Casting|CastToPlayerController (Pawn|GetController (Variables|Default|GetFirst%20PersonCharacter))))
  (Utilities|IsValid (PlayerController|LocalPlayerSubsystems|GetEnhancedInputLocalPlayerSubsystem _asplayer_controller)
    (:Is%20Valid
      (Input|AddMappingContext (PlayerController|LocalPlayerSubsystems|GetEnhancedInputLocalPlayerSubsystem _asplayer_controller) "/Game/NatsBlueprints/Input/IMC_Flamethrower.IMC_Flamethrower" 1 "(bIgnoreAllPressedKeysUntilRelease=True,bForceImmediately=False)")
      (Utilities|FlowControl|Delay 0.5)
      (Variables|Default|SetisToggling false))))

(event EventTick
  (params (DeltaSeconds :type Float%20%28single-precision%29))
  (bind _skeletalmeshref (Variables|Default|GetSkeletalMeshRef))
  (bind _first_personcharacter (Variables|Default|GetFirst%20PersonCharacter))
  ;[1 1 1] EventTickLogic
  (|CallParentFunction DeltaSeconds)
  (Utilities|FlowControl|DelayUntilNextTick)
  (if (Variables|Default|GetIsAttacking)
    (CallFunction|AmmoDrain 0.5 2.0)
    (if (<= (Variables|Default|GetammoAmount) 0.0)
      ;[1 0.01042 0.01042] Attack Logic (Left)
      ;;[1 1 1] Attack End
      (if (not (Variables|Default|GetisDisabling))
        (Variables|Default|SetisDisabling true)
        (Variables|/Game/NatsBlueprints/Blueprints/Player/BP_FirstPersonCharacter.BP_FirstPersonCharacter_C|SetisAttacking%28Player%29 _first_personcharacter false)
        (Variables|/Game/NatsBlueprints/Blueprints/Player/BP_FirstPersonCharacter.BP_FirstPersonCharacter_C|SetbFlamethrowerAttacking _first_personcharacter false)
        (Variables|Default|SetIsAttacking false)
        (Components|Animation|PlayAnimation _skeletalmeshref "/Game/Imports/Viewmodel_Testing/FPV_Spraycan/Spraycan_AttackEnd.Spraycan_AttackEnd" false)
        (Utilities|FlowControl|Delay 0.05)
        (Utilities|IsValid (stale Input|EnhancedActionEvents|EnhancedInputActionIA_SprayLeft _returnvalue)
          (:Is%20Valid
            (Variables|/Game/NatsBlueprints/Blueprints/Weapons/One-Handed/Spraycan/SpraycanHitboxParent.SpraycanHitboxParent_C|Setactive (stale Input|EnhancedActionEvents|EnhancedInputActionIA_SprayLeft _returnvalue) false))
          (:Is%20Not%20Valid
            _))
        (Utilities|FlowControl|Delay 0.05)
        (Components|Animation|PlayAnimation _skeletalmeshref "/Game/Imports/Viewmodel_Testing/FPV_Spraycan/Spraycan_CapIdle.Spraycan_CapIdle" true)
        (Variables|Default|SetisDisabling false)
        (Utilities|IsValid (stale Input|EnhancedActionEvents|EnhancedInputActionIA_SprayLeft _returnvalue_2)
          (:Is%20Valid
            (Audio|Components|Audio|Stop (stale Input|EnhancedActionEvents|EnhancedInputActionIA_SprayLeft _returnvalue_2))
            (Components|DestroyComponent (stale Input|EnhancedActionEvents|EnhancedInputActionIA_SprayLeft _returnvalue_2))))))
    (else
      ;[1 1 1] RechargeLogic
      (if (<= (Variables|Default|GetammoRechargeDelay) 0.0)
        (CallFunction|AmmoDrain -0.5 0.0))
      (Utilities|FlowControl|Delay 0.1)
      (Variables|Default|SetammoRechargeDelay (- (Variables|Default|GetammoRechargeDelay) 0.1)))))

(event EventUnequip
  (params (SpawnPickup :type Boolean))
  (bind _returnvalue (Transformation|GetWorldLocation))
  (bind _first_personcharacter (Variables|Default|GetFirst%20PersonCharacter))
  (bind _first_personcharacter_2 (Variables|Default|GetFirst%20PersonCharacter))
  (bind _first_personcharacter_3 (Variables|Default|GetFirst%20PersonCharacter))
  (bind _firstpersoncamera (Variables|/Game/NatsBlueprints/Blueprints/Player/BP_FirstPersonCharacter.BP_FirstPersonCharacter_C|GetFirstPersonCamera _first_personcharacter_2))
  (bind _returnvalue_2 (Transformation|GetWorldRotation _firstpersoncamera))
  (bind _returnvalue_3 (Math|Vector|GetForwardVector _returnvalue_2))
  (bind _returnvalue_4 (* _returnvalue_3 2.5e+04))
  (bind _returnvalue_5 (+ _returnvalue _returnvalue_4))
  ;[1 1 1] Unequip Logic
  (if SpawnPickup
    (bind _returnvalue_6 (Game|SpawnActorfromClass "/Game/NatsBlueprints/Blueprints/Weapons/Two-Handed/Spraycan_Lighter/BP_Flamethrower_Pickup.BP_Flamethrower_Pickup_C" (Transformation|GetActorTransform _first_personcharacter) "Undefined" "MultiplyWithRoot" 0 0))
    (Physics|AddForce (Variables|/Game/NatsBlueprints/Blueprints/Weapons/Two-Handed/Spraycan_Lighter/BP_Flamethrower_Pickup.BP_Flamethrower_Pickup_C|GetSkeletalMesh _returnvalue_6) _returnvalue_5 "None" true)
    (Physics|AddForce (Variables|/Game/NatsBlueprints/Blueprints/Weapons/Two-Handed/Spraycan_Lighter/BP_Flamethrower_Pickup.BP_Flamethrower_Pickup_C|GetSkeletalMesh1 _returnvalue_6) _returnvalue_5 "None" true))
  (Variables|/Game/NatsBlueprints/Blueprints/Player/BP_FirstPersonCharacter.BP_FirstPersonCharacter_C|SetbHasFlamethrower _first_personcharacter_3 false)
  (Variables|/Game/NatsBlueprints/Blueprints/Player/BP_FirstPersonCharacter.BP_FirstPersonCharacter_C|SetisCurrentWeaponTwoHanded? _first_personcharacter_3 false)
  (bind _asplayer_controller (Utilities|Casting|CastToPlayerController (Pawn|GetController _first_personcharacter))
    (:then
      (Utilities|IsValid (PlayerController|LocalPlayerSubsystems|GetEnhancedInputLocalPlayerSubsystem _asplayer_controller)
        (:Is%20Valid
          (Input|RemoveMappingContext (PlayerController|LocalPlayerSubsystems|GetEnhancedInputLocalPlayerSubsystem _asplayer_controller) "/Game/NatsBlueprints/Input/IMC_Flamethrower.IMC_Flamethrower" "(bIgnoreAllPressedKeysUntilRelease=True,bForceImmediately=False)"))
        (:Is%20Not%20Valid
          _)))
    (:CastFailed
      _))
  (Utilities|IsValid (stale Input|EnhancedActionEvents|EnhancedInputActionIA_SprayLeft _returnvalue)
    (:Is%20Valid
      (Actor|DestroyActor (stale Input|EnhancedActionEvents|EnhancedInputActionIA_SprayLeft _returnvalue)))
    (:Is%20Not%20Valid
      _))
  (Utilities|IsValid 0
    (:Is%20Not%20Valid
      (Utilities|IsValid (stale Input|EnhancedActionEvents|EnhancedInputActionIA_SprayLeft _returnvalue_2)
        (:Is%20Valid
          (Audio|Components|Audio|Stop (stale Input|EnhancedActionEvents|EnhancedInputActionIA_SprayLeft _returnvalue_2)))
        (:Is%20Not%20Valid
          _))
      (Utilities|IsValid 0
        (:Is%20Not%20Valid
          (Components|DestroyComponent)
          (Actor|DestroyActor (stale EventBeginPlay _returnvalue)))))))