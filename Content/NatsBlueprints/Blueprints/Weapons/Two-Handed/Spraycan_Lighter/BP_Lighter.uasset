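; BP_Lighter is a two-handed spraycan-and-lighter weapon Blueprint that shows or hides its Flame effect.
; On BeginPlay it caches the first-person player character and activates Flame after a short delay.
; Each tick it reads the character's LighterActive flag, re-activating Flame after the same delay when true and deactivating it immediately when false.
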(event EventBeginPlay
  (bind _asbp_first_person_character (Utilities|Casting|CastToBP_FirstPersonCharacter (Game|GetPlayerCharacter 0)))
  (Utilities|FlowControl|Delay 0.3)
  (Components|Activation|Activate (Variables|Default|GetFlame) false))

(event Collision|EventActorBeginOverlap
  (params (OtherActor :type Actor%20Object%20Reference)))

(event EventTick
  (params (DeltaSeconds :type Float%20%28single-precision%29))
  (if (Variables|/Game/NatsBlueprints/Blueprints/Player/BP_FirstPersonCharacter.BP_FirstPersonCharacter_C|GetbLighterActive (stale EventBeginPlay _asbp_first_person_character))
    (Utilities|FlowControl|Delay 0.3)
    (Components|Activation|Activate (Variables|Default|GetFlame) false)
    (else
      (Components|Activation|Deactivate (Variables|Default|GetFlame)))))

(fn ConstructionScript)