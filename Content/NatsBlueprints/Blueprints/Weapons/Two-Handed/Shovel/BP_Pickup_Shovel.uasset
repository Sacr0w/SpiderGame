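; Pickup actor for the two-handed Shovel weapon, initialising its info from the "Shovel" row on BeginPlay.
; On Pickup it either tags itself Stored and hides, or adds a shovel component to the first-person character as the equipped two-handed weapon and destroys itself.
; Tick swaps the mesh to a blue material while highlighted and keeps the info widget above the shovel, facing the player's view.
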(event EventBeginPlay
  (|CallParentFunction)
  (Variables|Default|SetInfoRow "Shovel")
  (CallFunction|InitialiseInfo)
  (Variables|Default|SetInfoScreenOffset "0.000000,0.000000,100.000000"))

(event EventPickup
  (params (PlayerRef :type BP%20First%20Person%20Character%20Object%20Reference) (LeftHanded :type Boolean) (Storing :type Boolean) (PickupFromStorage :type Boolean))
  ;[0.05 0.05 0.05] Pickup Logic
  (if (not (and (Actor|ActorHasTag self "Stored") (not PickupFromStorage)))
    (if Storing
      (Variables|Default|SetTags (Utilities|Array|MakeArray "Stored"))
      (Rendering|SetActorHiddenInGame true)
      (Collision|SetActorEnableCollision false)
      (else
        (bind _output_get (Variables|Default|SetFirstPersonCharacterReference PlayerRef))
        (bind _returnvalue (AddComponent|AddBPShovelComponent _output_get false))
        (Variables|/Game/NatsBlueprints/Blueprints/Player/BP_FirstPersonCharacter.BP_FirstPersonCharacter_C|SettwoHandedWeaponEquipped _output_get _returnvalue)
        (Actor|DestroyActor)))))

(event EventTick
  (params (DeltaSeconds :type Float%20%28single-precision%29))
  ;[0.03646 0.03646 0.03646] Highlight Logic
  (|CallParentFunction 0.0)
  (if (Variables|Default|GetHighlighted)
    (Rendering|Material|SetMaterial (Variables|Default|GetSkeletalMesh) 0 "/Game/LevelPrototyping/Materials/MI_Solid_Blue.MI_Solid_Blue")
    (else
      (Rendering|Material|SetMaterial (Variables|Default|GetSkeletalMesh) 0 "/Game/Assets/Materials/M_Shovel.M_Shovel")))
  (Transformation|SetWorldLocationAndRotation (Variables|Default|GetWeaponInfo) (+ (Transformation|GetWorldLocation (Variables|Default|GetSkeletalMesh)) (Variables|Default|GetInfoScreenOffset)) (Math|Rotator|FindLookatRotation (Transformation|GetWorldLocation (Variables|Default|GetWeaponInfo)) (.OutLocation (Actor|GetActorEyesViewPoint (Game|GetPlayerCharacter 0)))) false true))

(fn ConstructionScript)