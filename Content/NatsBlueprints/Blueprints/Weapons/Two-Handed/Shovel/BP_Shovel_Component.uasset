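; Two-handed shovel weapon component that attaches to the first-person character's mesh, occupies both hands and adds its own input mapping.
; Attacks play a montage whose Impact notify sphere-overlaps ahead of the camera, plays hit or miss audio and calls OnHit on animals, though DamageCalc has no logic.
; Blocking and attack flags are mirrored to the character.
; Unequip optionally throws a pickup, clears shovel state and destroys the component.
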(event Input|EnhancedActionEvents|EnhancedInputActionIA_Shoot
  (params (ActionValue :type Boolean) (ElapsedSeconds :type Float%20%28double-precision%29) (TriggeredSeconds :type Float%20%28double-precision%29) (InputAction :type Input%20Action%20Object%20Reference :default "/Game/NatsBlueprints/Input/Actions/IA_Shoot.IA_Shoot"))
  (bind _first_personcharacter (Variables|Default|GetFirst%20PersonCharacter))
  (bind _firstpersoncamera (Variables|/Game/NatsBlueprints/Blueprints/Player/BP_FirstPersonCharacter.BP_FirstPersonCharacter_C|GetFirstPersonCamera _first_personcharacter))
  ;[1 1 1] Attack Logic
  (:Triggered
    (if (not (Variables|Default|GetIsAttacking))
      (if (not (Variables|/Game/NatsBlueprints/Blueprints/Player/BP_FirstPersonCharacter.BP_FirstPersonCharacter_C|GetisKicking (Variables|Default|GetFirst%20PersonCharacter)))
        (if (not (Variables|Default|GetisBlocking))
          (Variables|Default|SetIsAttacking true)
          (Variables|/Game/NatsBlueprints/Blueprints/Player/BP_FirstPersonCharacter.BP_FirstPersonCharacter_C|SetisAttacking%28Player%29 (Variables|Default|GetFirst%20PersonCharacter) true)
          (bind _notifyname (Animation|Montage|PlayMontage (Variables|/Game/NatsBlueprints/Blueprints/Player/BP_FirstPersonCharacter.BP_FirstPersonCharacter_C|GetFirstPersonMesh (Variables|Default|GetFirst%20PersonCharacter)) "/Game/untitled_category/ShovelAttackMontage.ShovelAttackMontage")
            (:OnNotifyBegin
              (if (or (== _notifyname "Impact") (== _notifyname "IMPACT"))
                (bind _outactors (Actor|GetAllActorsOfClass "/Game/NatsBlueprints/Blueprints/Player/BP_FirstPersonCharacter.BP_FirstPersonCharacter_C"))
                (bind (_outactors_2 _returnvalue) (Collision|SphereOverlapActors (+ (Transformation|GetWorldLocation _firstpersoncamera) (* (Math|Vector|GetForwardVector (Transformation|GetWorldRotation _firstpersoncamera)) 1.2e+02)) 7e+01 (Variables|Default|GetObject%20Types) "/Game/Assets/Animals/Animal_Parent.Animal_Parent_C" _outactors))
                (if _returnvalue
                  (Audio|PlaySoundatLocation "/Game/Assets/Audio/Shovel_Hit_01.Shovel_Hit_01" "0, 0, 0" "0, 0, 0" 1.0 1.0 0.0 0 0 0 0)
                  (else
                    (Audio|PlaySoundatLocation "/Game/Assets/Audio/Shovel_Miss.Shovel_Miss" "0, 0, 0" "0, 0, 0" 1.0 1.0 0.0 0 0 0 0)))
                (for _array_element _outactors_2
                  (bind _asanimal_parent (Utilities|Casting|CastToAnimal_Parent _array_element))
                  (bind _finaldamage (CallFunction|DamageCalc (Variables|Default|GetDamage)))
                  (Default|OnHit _asanimal_parent _finaldamage))
                (else
                  (Variables|Default|SetIsAttacking false)
                  (Variables|/Game/NatsBlueprints/Blueprints/Player/BP_FirstPersonCharacter.BP_FirstPersonCharacter_C|SetisAttacking%28Player%29 (Variables|Default|GetFirst%20PersonCharacter) false))))))))))

(event Input|EnhancedActionEvents|EnhancedInputActionIA_Shovel_Block
  (params (ActionValue :type Boolean) (ElapsedSeconds :type Float%20%28double-precision%29) (TriggeredSeconds :type Float%20%28double-precision%29) (InputAction :type Input%20Action%20Object%20Reference :default "/Game/NatsBlueprints/Input/Actions/IA_Shovel_Block.IA_Shovel_Block"))
  ;[1 1 1] ShovelActivateLogic
  (:Triggered
    (if (not (Variables|Default|GetIsAttacking))
      (Variables|Default|SetisBlocking true)
      (Variables|/Game/NatsBlueprints/Blueprints/Player/BP_FirstPersonCharacter.BP_FirstPersonCharacter_C|SetisBlocking (Variables|Default|GetFirst%20PersonCharacter) true)))
  (:Completed
    (Variables|Default|SetisBlocking false)
    (Variables|/Game/NatsBlueprints/Blueprints/Player/BP_FirstPersonCharacter.BP_FirstPersonCharacter_C|SetisBlocking (Variables|Default|GetFirst%20PersonCharacter) false)))

(event EventBeginPlay
  ;[1 1 1] EquipLogic
  (bind _asbp_first_person_character (Utilities|Casting|CastToBP_FirstPersonCharacter (Components|GetOwner)))
  (bind _output_get (Variables|Default|SetFirst%20PersonCharacter _asbp_first_person_character))
  (Transformation|AttachComponentToComponent (Variables|/Game/NatsBlueprints/Blueprints/Player/BP_FirstPersonCharacter.BP_FirstPersonCharacter_C|GetFirstPersonMesh _output_get) "TwoHandedShovelPoint" "SnapToTarget" "SnapToTarget" "SnapToTarget" true)
  (Variables|/Game/NatsBlueprints/Blueprints/Player/BP_FirstPersonCharacter.BP_FirstPersonCharacter_C|SetbHasShovel (Variables|Default|GetFirst%20PersonCharacter) true)
  (Variables|/Game/NatsBlueprints/Blueprints/Player/BP_FirstPersonCharacter.BP_FirstPersonCharacter_C|SetleftHandAvailable (Variables|Default|GetFirst%20PersonCharacter) false)
  (Variables|/Game/NatsBlueprints/Blueprints/Player/BP_FirstPersonCharacter.BP_FirstPersonCharacter_C|SetrightHandAvailable (Variables|Default|GetFirst%20PersonCharacter) false)
  (Variables|/Game/NatsBlueprints/Blueprints/Player/BP_FirstPersonCharacter.BP_FirstPersonCharacter_C|SetisCurrentWeaponTwoHanded? (Variables|Default|GetFirst%20PersonCharacter) true)
  (bind _asplayer_controller (Utilities|Casting|CastToPlayerController (Pawn|GetController (Variables|Default|GetFirst%20PersonCharacter))))
  (Utilities|IsValid (PlayerController|LocalPlayerSubsystems|GetEnhancedInputLocalPlayerSubsystem _asplayer_controller)
    (:Is%20Valid
      (Input|AddMappingContext (PlayerController|LocalPlayerSubsystems|GetEnhancedInputLocalPlayerSubsystem _asplayer_controller) "/Game/NatsBlueprints/Input/IMC_Shovel.IMC_Shovel" 1 "(bIgnoreAllPressedKeysUntilRelease=True,bForceImmediately=False)"))))

(event EventUnequip
  (params (SpawnPickup :type Boolean))
  (bind _first_personcharacter (Variables|Default|GetFirst%20PersonCharacter))
  (bind _first_personcharacter_2 (Variables|Default|GetFirst%20PersonCharacter))
  ;[1 1 1] Unequip Logic
  (if SpawnPickup
    (bind _returnvalue (Game|SpawnActorfromClass "/Game/NatsBlueprints/Blueprints/Weapons/Two-Handed/Shovel/BP_Pickup_Shovel.BP_Pickup_Shovel_C" (Transformation|GetActorTransform _first_personcharacter) "Undefined" "MultiplyWithRoot" 0 0))
    (Physics|AddForce (Variables|/Game/NatsBlueprints/Blueprints/Weapons/Two-Handed/Shovel/BP_Pickup_Shovel.BP_Pickup_Shovel_C|GetSkeletalMesh _returnvalue) (+ (Transformation|GetWorldLocation) (* (Math|Vector|GetForwardVector (Transformation|GetWorldRotation (Variables|/Game/NatsBlueprints/Blueprints/Player/BP_FirstPersonCharacter.BP_FirstPersonCharacter_C|GetFirstPersonCamera (Variables|Default|GetFirst%20PersonCharacter)))) 2.5e+04)) "None" true))
  (Variables|/Game/NatsBlueprints/Blueprints/Player/BP_FirstPersonCharacter.BP_FirstPersonCharacter_C|SetbHasShovel _first_personcharacter_2 false)
  (Variables|/Game/NatsBlueprints/Blueprints/Player/BP_FirstPersonCharacter.BP_FirstPersonCharacter_C|SetisCurrentWeaponTwoHanded? _first_personcharacter_2 false)
  (bind _asplayer_controller (Utilities|Casting|CastToPlayerController (Pawn|GetController _first_personcharacter))
    (:then
      (Utilities|IsValid (PlayerController|LocalPlayerSubsystems|GetEnhancedInputLocalPlayerSubsystem _asplayer_controller)
        (:Is%20Valid
          (Input|RemoveMappingContext (PlayerController|LocalPlayerSubsystems|GetEnhancedInputLocalPlayerSubsystem _asplayer_controller) "/Game/NatsBlueprints/Input/IMC_Shovel.IMC_Shovel" "(bIgnoreAllPressedKeysUntilRelease=True,bForceImmediately=False)"))
        (:Is%20Not%20Valid
          _)))
    (:CastFailed
      _))
  (Components|DestroyComponent))