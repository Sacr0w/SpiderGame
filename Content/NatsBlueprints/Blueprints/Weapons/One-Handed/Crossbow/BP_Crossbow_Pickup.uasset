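; BP_Crossbow_Pickup is a pickup actor that equips a crossbow on the first-person player character.
; Its Pickup event adds a BP Crossbow component to the player, assigns it as the left or right equipped weapon, initializes it through OnCreate, then destroys the actor.
; Tick sets the skeletal mesh to a solid blue material while highlighted, otherwise to its base material.
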(event EventBeginPlay
  (|CallParentFunction) ; This node is disabled and will not be called.\nDrag off pins to build functionality.
)

(event EventPickup
  (params (PlayerRef :type BP%20First%20Person%20Character%20Object%20Reference) (LeftHanded :type Boolean))
  (bind _output_get (Variables|Default|SetFirstPersonCharacterRef PlayerRef))
  (bind _returnvalue (AddComponent|AddBPCrossbowComponent _output_get false))
  (if LeftHanded
    (Variables|/Game/NatsBlueprints/Blueprints/BP_FirstPersonCharacter.BP_FirstPersonCharacter_C|SetleftWeaponEquipped _output_get _returnvalue)
    (else
      (Variables|/Game/NatsBlueprints/Blueprints/BP_FirstPersonCharacter.BP_FirstPersonCharacter_C|SetrightWeaponEquipped _output_get _returnvalue)))
  (Default|OnCreate _returnvalue LeftHanded)
  (Actor|DestroyActor))

(event EventTick
  (params (DeltaSeconds :type Float%20%28single-precision%29))
  (bind _skeletalmesh (Variables|Default|GetSkeletalMesh))
  (if (Variables|Default|GetHighlighted)
    (Rendering|Material|SetMaterial _skeletalmesh 0 "/Game/LevelPrototyping/Materials/MI_Solid_Blue.MI_Solid_Blue")
    (else
      (Rendering|Material|SetMaterial _skeletalmesh 0 "/Game/FPWeapon/Materials/BaseMaterial.BaseMaterial"))))

(event Collision|EventActorBeginOverlap
  (params (OtherActor :type Actor%20Object%20Reference))
  (|CallParentFunction OtherActor) ; This node is disabled and will not be called.\nDrag off pins to build functionality.
)

(fn ConstructionScript
  (|CallParentFunction))