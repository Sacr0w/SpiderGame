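; Crossbow weapon component that equips to the first-person character's left or right hand and fires projectiles.
; OnCreate snaps it to the hand socket, flags the crossbow and occupied hand on the character, and adds that hand's Enhanced Input mapping context.
; IA_Shoot spawns a projectile at the character's actor transform.
; Unequip spawns a pickup, clears only the crossbow flag, removes both mapping contexts and destroys the component.
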(event Input|EnhancedActionEvents|EnhancedInputActionIA_Shoot
  (params (ActionValue :type Boolean) (ElapsedSeconds :type Float%20%28double-precision%29) (TriggeredSeconds :type Float%20%28double-precision%29) (InputAction :type Input%20Action%20Object%20Reference :default "/Game/NatsBlueprints/Input/Actions/IA_Shoot.IA_Shoot"))
  (:Triggered
    (Game|SpawnActorfromClass "/Game/NatsBlueprints/Blueprints/BP_FirstPersonProjectile.BP_FirstPersonProjectile_C" (Transformation|GetActorTransform (Variables|Default|GetFirst%20PersonCharacter)) "Undefined" "MultiplyWithRoot" 0 0)))

(event EventTick
  (params (DeltaSeconds :type Float%20%28single-precision%29))
  (|CallParentFunction DeltaSeconds) ; This node is disabled and will not be called.\nDrag off pins to build functionality.
)

(event EventOnCreate
  (params (LeftHanded :type Boolean))
  (bind _output_get (Variables|Default|SetLeftHanded LeftHanded))
  (bind _asbp_first_person_character (Utilities|Casting|CastToBP_FirstPersonCharacter (Components|GetOwner)))
  (bind _output_get_2 (Variables|Default|SetFirst%20PersonCharacter _asbp_first_person_character))
  (Transformation|AttachComponentToComponent (Variables|/Game/NatsBlueprints/Blueprints/BP_FirstPersonCharacter.BP_FirstPersonCharacter_C|GetFirstPersonMesh _output_get_2) (select _output_get "LeftHandPoint" "RightHandPoint") "SnapToTarget" "SnapToTarget" "SnapToTarget" true)
  (Variables|/Game/NatsBlueprints/Blueprints/BP_FirstPersonCharacter.BP_FirstPersonCharacter_C|SetbHasCrossbow (Variables|Default|GetFirst%20PersonCharacter) true)
  (if (Variables|Default|GetLeftHanded)
    (Variables|/Game/NatsBlueprints/Blueprints/BP_FirstPersonCharacter.BP_FirstPersonCharacter_C|SetleftHandAvailable (Variables|Default|GetFirst%20PersonCharacter) false)
    (else
      (Variables|/Game/NatsBlueprints/Blueprints/BP_FirstPersonCharacter.BP_FirstPersonCharacter_C|SetrightHandAvailable (Variables|Default|GetFirst%20PersonCharacter) false)))
  (bind _asplayer_controller (Utilities|Casting|CastToPlayerController (Pawn|GetController (Variables|Default|GetFirst%20PersonCharacter))))
  (Utilities|IsValid (PlayerController|LocalPlayerSubsystems|GetEnhancedInputLocalPlayerSubsystem _asplayer_controller)
    (:Is%20Valid
      (if (Variables|Default|GetLeftHanded)
        (Input|AddMappingContext (PlayerController|LocalPlayerSubsystems|GetEnhancedInputLocalPlayerSubsystem _asplayer_controller) "/Game/NatsBlueprints/Input/IMC_Crossbow_Left.IMC_Crossbow_Left" 1 "(bIgnoreAllPressedKeysUntilRelease=True,bForceImmediately=False)")
        (else
          (Input|AddMappingContext (PlayerController|LocalPlayerSubsystems|GetEnhancedInputLocalPlayerSubsystem _asplayer_controller) "/Game/NatsBlueprints/Input/IMC_Crossbow_Right.IMC_Crossbow_Right" 1 "(bIgnoreAllPressedKeysUntilRelease=True,bForceImmediately=False)"))))))

(event EventUnequip
  (bind _first_personcharacter (Variables|Default|GetFirst%20PersonCharacter))
  (Game|SpawnActorfromClass "/Game/NatsBlueprints/Blueprints/Weapons/One-Handed/Crossbow/BP_Crossbow_Pickup.BP_Crossbow_Pickup_C" (Transformation|GetActorTransform _first_personcharacter) "Undefined" "MultiplyWithRoot" 0 0)
  (Variables|/Game/NatsBlueprints/Blueprints/BP_FirstPersonCharacter.BP_FirstPersonCharacter_C|SetbHasCrossbow (Variables|Default|GetFirst%20PersonCharacter) false)
  (bind _asplayer_controller (Utilities|Casting|CastToPlayerController (Pawn|GetController _first_personcharacter))
    (:then
      (Utilities|IsValid (PlayerController|LocalPlayerSubsystems|GetEnhancedInputLocalPlayerSubsystem _asplayer_controller)
        (:Is%20Valid
          (Input|RemoveMappingContext (PlayerController|LocalPlayerSubsystems|GetEnhancedInputLocalPlayerSubsystem _asplayer_controller) "/Game/NatsBlueprints/Input/IMC_Crossbow_Left.IMC_Crossbow_Left" "(bIgnoreAllPressedKeysUntilRelease=True,bForceImmediately=False)")
          (Input|RemoveMappingContext (PlayerController|LocalPlayerSubsystems|GetEnhancedInputLocalPlayerSubsystem _asplayer_controller) "/Game/NatsBlueprints/Input/IMC_Crossbow_Right.IMC_Crossbow_Right" "(bIgnoreAllPressedKeysUntilRelease=True,bForceImmediately=False)"))
        (:Is%20Not%20Valid
          _)))
    (:CastFailed
      _))
  (Components|DestroyComponent))