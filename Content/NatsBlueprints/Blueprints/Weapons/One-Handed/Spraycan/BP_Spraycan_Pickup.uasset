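; Weapon pickup for the one-handed spraycan, with a B variant chosen when its second upgrade amount is above zero, changing its info row and material.
; Pickup either hides the actor as stored or adds a spraycan component to the player's left or right hand, passes on upgrades and destroys itself.
; Tick swaps materials for highlighting and turns the floating info screen toward the player's view.
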(event EventBeginPlay
  (|CallParentFunction)
  (Utilities|FlowControl|Delay 0.01)
  (if (> (Variables|Default|GetupgradeAmount%28B%29) 0)
    (Variables|Default|SetInfoRow "Spraycan-B"))
  (CallFunction|InitialiseInfo 0.0))

(event EventPickup
  (params (PlayerRef :type BP%20First%20Person%20Character%20Object%20Reference) (LeftHanded :type Boolean) (Storing :type Boolean) (PickupFromStorage :type Boolean))
  (|CallParentFunction 0 LeftHanded Storing PickupFromStorage)
  (if (not (and (Actor|ActorHasTag "Stored") (not PickupFromStorage)))
    (if Storing
      (Variables|Default|SetTags (Utilities|Array|MakeArray "Stored"))
      (Rendering|SetActorHiddenInGame true)
      (Collision|SetActorEnableCollision false)
      (else
        (bind _output_get (Variables|Default|SetFirstPersonCharacterRef PlayerRef))
        (bind _returnvalue (AddComponent|AddBPSpraycanComponent _output_get false))
        (if LeftHanded
          (Variables|/Game/NatsBlueprints/Blueprints/Player/BP_FirstPersonCharacter.BP_FirstPersonCharacter_C|SetleftWeaponEquipped _output_get _returnvalue)
          (else
            (Variables|/Game/NatsBlueprints/Blueprints/Player/BP_FirstPersonCharacter.BP_FirstPersonCharacter_C|SetrightWeaponEquipped _output_get _returnvalue)))
        (if LeftHanded
          (Variables|/Game/NatsBlueprints/Blueprints/Player/BP_FirstPersonCharacter.BP_FirstPersonCharacter_C|SetbHasLeftHandedSpraycan _output_get true)
          (else
            (Variables|/Game/NatsBlueprints/Blueprints/Player/BP_FirstPersonCharacter.BP_FirstPersonCharacter_C|SetbHasRightHandedSpraycan _output_get true)))
        (Variables|/Game/NatsBlueprints/Blueprints/Weapons/BP_WeaponFunction_Parent.BP_WeaponFunction_Parent_C|SetupgradeAmount%281%29 _returnvalue (Variables|Default|GetupgradeAmount%28A%29))
        (Variables|/Game/NatsBlueprints/Blueprints/Weapons/BP_WeaponFunction_Parent.BP_WeaponFunction_Parent_C|SetupgradeAmount%282%29 _returnvalue (Variables|Default|GetupgradeAmount%28B%29))
        (Default|OnCreate _returnvalue LeftHanded _returnvalue)
        (Audio|PlaySound2D "/Game/NatsBlueprints/Blueprints/Weapons/One-Handed/Spraycan/SpraycanEquip.SpraycanEquip" 1.0 1.0 0.0 0 0)
        (Actor|DestroyActor)))))

(event EventTick
  (params (DeltaSeconds :type Float%20%28single-precision%29))
  (bind _skeletalmesh (Variables|Default|GetSkeletalMesh))
  (|CallParentFunction 0.0)
  (if (Variables|Default|GetHighlighted)
    (Rendering|Material|SetMaterial _skeletalmesh 0 "/Game/LevelPrototyping/Materials/MI_Solid_Blue.MI_Solid_Blue")
    (else
      (Rendering|Material|SetMaterial _skeletalmesh 0 (select (> (Variables|Default|GetupgradeAmount%28B%29) 0) "/AnimationSharing/AnimSharingGreen.AnimSharingGreen" "/Game/Imports/Viewmodel_Testing/FPV_Spraycan/M_Bugspray_Texture.M_Bugspray_Texture"))
      (Rendering|Material|SetMaterial _skeletalmesh 1 "/Game/Imports/Viewmodel_Testing/FPV_Spraycan/Outline.Outline")))
  (Transformation|SetWorldLocationAndRotation (Variables|Default|GetWeaponInfo) (+ (Transformation|GetWorldLocation (Variables|Default|GetSkeletalMesh)) (Variables|Default|GetInfoScreenOffset)) (Math|Rotator|FindLookatRotation (Transformation|GetWorldLocation (Variables|Default|GetWeaponInfo)) (.OutLocation (Actor|GetActorEyesViewPoint (Game|GetPlayerCharacter 0)))) false true))

(event Collision|EventActorBeginOverlap
  (params (OtherActor :type Actor%20Object%20Reference))
  (|CallParentFunction OtherActor) ; This node is disabled and will not be called.\nDrag off pins to build functionality.
)

(fn ConstructionScript
  (|CallParentFunction))