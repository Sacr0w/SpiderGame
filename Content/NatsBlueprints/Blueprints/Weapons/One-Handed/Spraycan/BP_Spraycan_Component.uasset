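; Weapon component for a one-handed spraycan that attaches to either hand of the first-person character and adds that hand's input mapping.
; Holding spray plays animations and sound and spawns an attached particle hitbox with calculated damage, plus poison when upgraded.
; Tick drains ammo while spraying, stops at empty and recharges after a delay.
; Unequip can throw a pickup preserving the upgrade level; one upgrade type instead unequips both hands.
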(event Input|EnhancedActionEvents|EnhancedInputActionIA_SprayLeft
  (params (ActionValue :type Boolean) (ElapsedSeconds :type Float%20%28double-precision%29) (TriggeredSeconds :type Float%20%28double-precision%29) (InputAction :type Input%20Action%20Object%20Reference :default "/Game/NatsBlueprints/Input/Actions/IA_SprayLeft.IA_SprayLeft"))
  (bind _upgradeamount_2_ (Variables|Default|GetupgradeAmount%282%29))
  (bind _first_personcharacter (Variables|Default|GetFirst%20PersonCharacter))
  (bind _skeletalmeshref (Variables|Default|GetSkeletalMeshRef))
  (bind _first_personcharacter_2 (Variables|Default|GetFirst%20PersonCharacter))
  ;[1 0.01042 0.01042] Attack Logic (Left)
  ;;[1 1 1] Attack Start
  (:Triggered
    (if (> (Variables|Default|GetammoAmount) 1e+01)
      (if (Variables|Default|GetLeftHanded)
        (if (not (Variables|Default|GetIsAttacking))
          (if (not (Variables|Default|GetisDisabling))
            (Variables|/Game/NatsBlueprints/Blueprints/Player/BP_FirstPersonCharacter.BP_FirstPersonCharacter_C|SetisAttacking%28Player%29 _first_personcharacter true)
            (if (stale EventOnCreate LeftHanded)
              (Variables|/Game/NatsBlueprints/Blueprints/Player/BP_FirstPersonCharacter.BP_FirstPersonCharacter_C|SetbLeftHandedSpraycanAttacking _first_personcharacter true)
              (else
                (Variables|/Game/NatsBlueprints/Blueprints/Player/BP_FirstPersonCharacter.BP_FirstPersonCharacter_C|SetbRightHandedSpraycanAttacking _first_personcharacter true)))
            (Variables|Default|SetIsAttacking true)
            (Components|Animation|PlayAnimation _skeletalmeshref "/Game/Imports/Viewmodel_Testing/FPV_Spraycan/Spraycan_AttackStart.Spraycan_AttackStart" false)
            (Utilities|FlowControl|Delay 0.05)
            (Components|Animation|PlayAnimation _skeletalmeshref "/Game/Imports/Viewmodel_Testing/FPV_Spraycan/Spraycan_AttackLoop.Spraycan_AttackLoop" true)
            (bind _returnvalue (Game|SpawnActorfromClass "/Game/NatsBlueprints/Blueprints/Weapons/One-Handed/Spraycan/SpraycanParticleHitbox.SpraycanParticleHitbox_C" (Transformation|GetWorldTransform) "Undefined" "MultiplyWithRoot" 0 0))
            (Transformation|AttachComponentToComponent _returnvalue self "CapSocket" "SnapToTarget" "SnapToTarget" "SnapToTarget" true)
            (if (> _upgradeamount_2_ 0)
              (Variables|/Game/NatsBlueprints/Blueprints/Weapons/One-Handed/Spraycan/SpraycanParticleHitbox.SpraycanParticleHitbox_C|SetAppliesPoison _returnvalue _upgradeamount_2_))
            (bind _finaldamage (CallFunction|DamageCalc (Variables|Default|GetbaseDamage) (Variables|Default|GetWeaponBaseDamagePercent)))
            (Variables|/Game/NatsBlueprints/Blueprints/Weapons/One-Handed/Spraycan/SpraycanHitboxParent.SpraycanHitboxParent_C|SetDamage _returnvalue _finaldamage)
            (bind _returnvalue_2 (Audio|CreateSound2D "/Game/NatsBlueprints/Blueprints/Weapons/One-Handed/Spraycan/Spraycan_Attack.Spraycan_Attack" 1.0 1.0 0.0 0))
            (Audio|Components|Audio|Play _returnvalue_2 0.0))))))
  (:Canceled
    ;;[1 1 1] Attack End
    (if (Variables|Default|GetLeftHanded) :!label _label
      (if (Variables|Default|GetIsAttacking)
        (if (not (Variables|Default|GetisDisabling))
          (Variables|Default|SetisDisabling true)
          (Variables|/Game/NatsBlueprints/Blueprints/Player/BP_FirstPersonCharacter.BP_FirstPersonCharacter_C|SetisAttacking%28Player%29 _first_personcharacter_2 false)
          (if (stale EventOnCreate LeftHanded)
            (Variables|/Game/NatsBlueprints/Blueprints/Player/BP_FirstPersonCharacter.BP_FirstPersonCharacter_C|SetbLeftHandedSpraycanAttacking _first_personcharacter_2 false)
            (else
              (Variables|/Game/NatsBlueprints/Blueprints/Player/BP_FirstPersonCharacter.BP_FirstPersonCharacter_C|SetbRightHandedSpraycanAttacking _first_personcharacter_2 false)))
          (Variables|Default|SetIsAttacking false)
          (Components|Animation|PlayAnimation _skeletalmeshref "/Game/Imports/Viewmodel_Testing/FPV_Spraycan/Spraycan_AttackEnd.Spraycan_AttackEnd" false)
          (Utilities|FlowControl|Delay 0.05)
          (Utilities|IsValid _returnvalue
            (:Is%20Valid
              (Variables|/Game/NatsBlueprints/Blueprints/Weapons/One-Handed/Spraycan/SpraycanHitboxParent.SpraycanHitboxParent_C|Setactive _returnvalue false))
            (:Is%20Not%20Valid
              _))
          (Utilities|FlowControl|Delay 0.05)
          (Components|Animation|PlayAnimation _skeletalmeshref "/Game/Imports/Viewmodel_Testing/FPV_Spraycan/Spraycan_CapIdle.Spraycan_CapIdle" true)
          (Variables|Default|SetisDisabling false)
          (Utilities|IsValid _returnvalue_2
            (:Is%20Valid
              (Audio|Components|Audio|Stop _returnvalue_2)
              (Components|DestroyComponent _returnvalue_2)))))))
  (:Completed
    (goto _label)))

(event Input|EnhancedActionEvents|EnhancedInputActionIA_SprayRight
  (params (ActionValue :type Boolean) (ElapsedSeconds :type Float%20%28double-precision%29) (TriggeredSeconds :type Float%20%28double-precision%29) (InputAction :type Input%20Action%20Object%20Reference :default "/Game/NatsBlueprints/Input/Actions/IA_SprayRight.IA_SprayRight"))
  (bind _upgradeamount_2_ (Variables|Default|GetupgradeAmount%282%29))
  (bind _first_personcharacter (Variables|Default|GetFirst%20PersonCharacter))
  (bind _lefthanded (Variables|Default|GetLeftHanded))
  (bind _first_personcharacter_2 (Variables|Default|GetFirst%20PersonCharacter))
  (bind _skeletalmeshref (Variables|Default|GetSkeletalMeshRef))
  ;[1 0.01042 0.01042] Attack Logic (Right)
  ;;[1 1 1] Attack Start
  (:Triggered
    (if (> (Variables|Default|GetammoAmount) 1e+01)
      (if (not (Variables|Default|GetLeftHanded))
        (if (not (Variables|Default|GetIsAttacking))
          (if (not (Variables|/Game/NatsBlueprints/Blueprints/Player/BP_FirstPersonCharacter.BP_FirstPersonCharacter_C|GetisKicking (Variables|Default|GetFirst%20PersonCharacter)))
            (if (not (Variables|Default|GetisDisabling))
              (if _lefthanded
                (Variables|/Game/NatsBlueprints/Blueprints/Player/BP_FirstPersonCharacter.BP_FirstPersonCharacter_C|SetbLeftHandedSpraycanAttacking _first_personcharacter_2 true)
                (else
                  (Variables|/Game/NatsBlueprints/Blueprints/Player/BP_FirstPersonCharacter.BP_FirstPersonCharacter_C|SetbRightHandedSpraycanAttacking _first_personcharacter_2 true)))
              (Variables|Default|SetIsAttacking true)
              (Components|Animation|PlayAnimation _skeletalmeshref "/Game/Imports/Viewmodel_Testing/FPV_Spraycan/Spraycan_AttackStart.Spraycan_AttackStart" false)
              (Utilities|FlowControl|Delay 0.05)
              (Components|Animation|PlayAnimation _skeletalmeshref "/Game/Imports/Viewmodel_Testing/FPV_Spraycan/Spraycan_AttackLoop.Spraycan_AttackLoop" true)
              (bind _returnvalue (Game|SpawnActorfromClass "/Game/NatsBlueprints/Blueprints/Weapons/One-Handed/Spraycan/SpraycanParticleHitbox.SpraycanParticleHitbox_C" (Transformation|GetWorldTransform) "Undefined" "MultiplyWithRoot" 0 0))
              (Transformation|AttachComponentToComponent _returnvalue self "CapSocket" "SnapToTarget" "SnapToTarget" "SnapToTarget" true)
              (if (> _upgradeamount_2_ 0)
                (Variables|/Game/NatsBlueprints/Blueprints/Weapons/One-Handed/Spraycan/SpraycanParticleHitbox.SpraycanParticleHitbox_C|SetAppliesPoison _returnvalue _upgradeamount_2_))
              (bind _finaldamage (CallFunction|DamageCalc (Variables|Default|GetbaseDamage) (Variables|Default|GetWeaponBaseDamagePercent)))
              (Variables|/Game/NatsBlueprints/Blueprints/Weapons/One-Handed/Spraycan/SpraycanHitboxParent.SpraycanHitboxParent_C|SetDamage _returnvalue _finaldamage)
              (bind _returnvalue_2 (Audio|CreateSound2D "/Game/NatsBlueprints/Blueprints/Weapons/One-Handed/Spraycan/Spraycan_Attack.Spraycan_Attack" 1.0 1.0 0.0 0))
              (Audio|Components|Audio|Play _returnvalue_2 0.0)))))))
  (:Canceled
    ;;[1 1 1] Attack End
    (if (not (Variables|Default|GetLeftHanded)) :!label _label
      (if (Variables|Default|GetIsAttacking)
        (if (not (Variables|Default|GetisDisabling))
          (Variables|/Game/NatsBlueprints/Blueprints/Player/BP_FirstPersonCharacter.BP_FirstPersonCharacter_C|SetisAttacking%28Player%29 (Variables|Default|GetFirst%20PersonCharacter) false)
          (Variables|Default|SetisDisabling true)
          (if _lefthanded
            (Variables|/Game/NatsBlueprints/Blueprints/Player/BP_FirstPersonCharacter.BP_FirstPersonCharacter_C|SetbLeftHandedSpraycanAttacking _first_personcharacter false)
            (else
              (Variables|/Game/NatsBlueprints/Blueprints/Player/BP_FirstPersonCharacter.BP_FirstPersonCharacter_C|SetbRightHandedSpraycanAttacking _first_personcharacter false)))
          (Variables|Default|SetIsAttacking false)
          (Components|Animation|PlayAnimation _skeletalmeshref "/Game/Imports/Viewmodel_Testing/FPV_Spraycan/Spraycan_AttackEnd.Spraycan_AttackEnd" false)
          (Utilities|FlowControl|Delay 0.05)
          (Utilities|IsValid _returnvalue
            (:Is%20Valid
              (Variables|/Game/NatsBlueprints/Blueprints/Weapons/One-Handed/Spraycan/SpraycanHitboxParent.SpraycanHitboxParent_C|Setactive _returnvalue false))
            (:Is%20Not%20Valid
              _))
          (Utilities|FlowControl|Delay 0.05)
          (Components|Animation|PlayAnimation _skeletalmeshref "/Game/Imports/Viewmodel_Testing/FPV_Spraycan/Spraycan_CapIdle.Spraycan_CapIdle" true)
          (Variables|Default|SetisDisabling false)
          (Utilities|IsValid _returnvalue_2
            (:Is%20Valid
              (Audio|Components|Audio|Stop _returnvalue_2)
              (Components|DestroyComponent _returnvalue_2)))))))
  (:Completed
    (goto _label)))

(event EventOnUpgrade
  (params (Upgrade%20#1 :type Boolean))
  (bind _first_personcharacter (Variables|Default|GetFirst%20PersonCharacter))
  (if Upgrade%20#1
    (if (Variables|Default|GetLeftHanded)
      (Default|Unequip(RightHand) _first_personcharacter)
      (else
        (Default|Unequip(LeftHand) _first_personcharacter)))
    (CallFunction|Unequip false)
    (else
      (Variables|Default|SetupgradeAmount%282%29 (+ (Variables|Default|GetupgradeAmount%282%29) 1))
      (Rendering|Material|SetMaterial (Variables|Default|GetSkeletalMeshRef) 0 (select (> (Variables|Default|GetupgradeAmount%282%29) 0) "/AnimationSharing/AnimSharingGreen.AnimSharingGreen" "/Game/Imports/Viewmodel_Testing/FPV_Spraycan/M_Bugspray_Texture.M_Bugspray_Texture")))))

(event EventTick
  (params (DeltaSeconds :type Float%20%28single-precision%29))
  (bind _first_personcharacter (Variables|Default|GetFirst%20PersonCharacter))
  (bind _skeletalmeshref (Variables|Default|GetSkeletalMeshRef))
  (bind _first_personcharacter_2 (Variables|Default|GetFirst%20PersonCharacter))
  (bind _skeletalmeshref_2 (Variables|Default|GetSkeletalMeshRef))
  ;[1 1 1] EventTickLogic
  (|CallParentFunction DeltaSeconds)
  (Utilities|FlowControl|DelayUntilNextTick)
  (if (Variables|Default|GetIsAttacking)
    (CallFunction|AmmoDrain 0.5 2.0)
    (if (<= (Variables|Default|GetammoAmount) 0.0)
      (if (Variables|Default|GetLeftHanded)
        ;[1 0.01042 0.01042] Attack Logic (Left)
        ;;[1 1 1] Attack End
        (if (not (Variables|Default|GetisDisabling))
          (Variables|Default|SetisDisabling true)
          (Variables|/Game/NatsBlueprints/Blueprints/Player/BP_FirstPersonCharacter.BP_FirstPersonCharacter_C|SetisAttacking%28Player%29 _first_personcharacter_2 false)
          (if (stale EventOnCreate LeftHanded)
            (Variables|/Game/NatsBlueprints/Blueprints/Player/BP_FirstPersonCharacter.BP_FirstPersonCharacter_C|SetbLeftHandedSpraycanAttacking _first_personcharacter_2 false)
            (else
              (Variables|/Game/NatsBlueprints/Blueprints/Player/BP_FirstPersonCharacter.BP_FirstPersonCharacter_C|SetbRightHandedSpraycanAttacking _first_personcharacter_2 false)))
          (Variables|Default|SetIsAttacking false)
          (Components|Animation|PlayAnimation _skeletalmeshref "/Game/Imports/Viewmodel_Testing/FPV_Spraycan/Spraycan_AttackEnd.Spraycan_AttackEnd" false)
          (Utilities|FlowControl|Delay 0.05)
          (Utilities|IsValid (stale Input|EnhancedActionEvents|EnhancedInputActionIA_SprayLeft _returnvalue)
            (:Is%20Valid
              (Variables|/Game/NatsBlueprints/Blueprints/Weapons/One-Handed/Spraycan/SpraycanHitboxParent.SpraycanHitboxParent_C|Setactive (stale Input|EnhancedActionEvents|EnhancedInputActionIA_SprayLeft _returnvalue) false))
            (:Is%20Not%20Valid
              _))
          (Utilities|FlowControl|Delay 0.05)
          (Components|Animation|PlayAnimation _skeletalmeshref "/Game/Imports/Viewmodel_Testing/FPV_Spraycan/Spraycan_CapIdle.Spraycan_CapIdle" true)
          (Variables|Default|SetisDisabling false)
          (Utilities|IsValid (stale Input|EnhancedActionEvents|EnhancedInputActionIA_SprayLeft _returnvalue_2)
            (:Is%20Valid
              (Audio|Components|Audio|Stop (stale Input|EnhancedActionEvents|EnhancedInputActionIA_SprayLeft _returnvalue_2))
              (Components|DestroyComponent (stale Input|EnhancedActionEvents|EnhancedInputActionIA_SprayLeft _returnvalue_2)))))
        (else
          ;[1 0.01042 0.01042] Attack Logic (Right)
          ;;[1 1 1] Attack End
          (if (not (Variables|Default|GetisDisabling))
            (Variables|/Game/NatsBlueprints/Blueprints/Player/BP_FirstPersonCharacter.BP_FirstPersonCharacter_C|SetisAttacking%28Player%29 (Variables|Default|GetFirst%20PersonCharacter) false)
            (Variables|Default|SetisDisabling true)
            (if (Variables|Default|GetLeftHanded)
              (Variables|/Game/NatsBlueprints/Blueprints/Player/BP_FirstPersonCharacter.BP_FirstPersonCharacter_C|SetbLeftHandedSpraycanAttacking _first_personcharacter false)
              (else
                (Variables|/Game/NatsBlueprints/Blueprints/Player/BP_FirstPersonCharacter.BP_FirstPersonCharacter_C|SetbRightHandedSpraycanAttacking _first_personcharacter false)))
            (Variables|Default|SetIsAttacking false)
            (Components|Animation|PlayAnimation _skeletalmeshref_2 "/Game/Imports/Viewmodel_Testing/FPV_Spraycan/Spraycan_AttackEnd.Spraycan_AttackEnd" false)
            (Utilities|FlowControl|Delay 0.05)
            (Utilities|IsValid (stale Input|EnhancedActionEvents|EnhancedInputActionIA_SprayRight _returnvalue)
              (:Is%20Valid
                (Variables|/Game/NatsBlueprints/Blueprints/Weapons/One-Handed/Spraycan/SpraycanHitboxParent.SpraycanHitboxParent_C|Setactive (stale Input|EnhancedActionEvents|EnhancedInputActionIA_SprayRight _returnvalue) false))
              (:Is%20Not%20Valid
                _))
            (Utilities|FlowControl|Delay 0.05)
            (Components|Animation|PlayAnimation _skeletalmeshref_2 "/Game/Imports/Viewmodel_Testing/FPV_Spraycan/Spraycan_CapIdle.Spraycan_CapIdle" true)
            (Variables|Default|SetisDisabling false)
            (Utilities|IsValid (stale Input|EnhancedActionEvents|EnhancedInputActionIA_SprayRight _returnvalue_2)
              (:Is%20Valid
                (Audio|Components|Audio|Stop (stale Input|EnhancedActionEvents|EnhancedInputActionIA_SprayRight _returnvalue_2))
                (Components|DestroyComponent (stale Input|EnhancedActionEvents|EnhancedInputActionIA_SprayRight _returnvalue_2))))))))
    (else
      ;[1 1 1] RechargeLogic
      (if (<= (Variables|Default|GetammoRechargeDelay) 0.0)
        (CallFunction|AmmoDrain -0.5 0.0))
      (Utilities|FlowControl|Delay 0.1)
      (Variables|Default|SetammoRechargeDelay (- (Variables|Default|GetammoRechargeDelay) 0.1)))))

(event EventOnCreate
  (params (LeftHanded :type Boolean) (SkeletalMeshRef :type Skeletal%20Mesh%20Component%20Object%20Reference))
  ;[1 1 1] Equip Logic
  (bind _output_get (Variables|Default|SetLeftHanded LeftHanded))
  (Variables|Default|SetSkeletalMeshRef SkeletalMeshRef)
  (bind _asbp_first_person_character (Utilities|Casting|CastToBP_FirstPersonCharacter (Components|GetOwner)))
  (bind _output_get_2 (Variables|Default|SetFirst%20PersonCharacter _asbp_first_person_character))
  (Transformation|AttachComponentToComponent (Variables|/Game/NatsBlueprints/Blueprints/Player/BP_FirstPersonCharacter.BP_FirstPersonCharacter_C|GetFirstPersonMesh _output_get_2) (select _output_get "LeftHandedSpraycanPoint" "RightHandedSpraycanPoint") "SnapToTarget" "SnapToTarget" "SnapToTarget" true)
  (if (Variables|Default|GetLeftHanded)
    (Variables|/Game/NatsBlueprints/Blueprints/Player/BP_FirstPersonCharacter.BP_FirstPersonCharacter_C|SetbHasLeftHandedSpraycan (Variables|Default|GetFirst%20PersonCharacter) true)
    (else
      (Variables|/Game/NatsBlueprints/Blueprints/Player/BP_FirstPersonCharacter.BP_FirstPersonCharacter_C|SetbHasRightHandedSpraycan (Variables|Default|GetFirst%20PersonCharacter) true)))
  (if (Variables|Default|GetLeftHanded)
    (Variables|/Game/NatsBlueprints/Blueprints/Player/BP_FirstPersonCharacter.BP_FirstPersonCharacter_C|SetleftHandAvailable (Variables|Default|GetFirst%20PersonCharacter) false)
    (else
      (Variables|/Game/NatsBlueprints/Blueprints/Player/BP_FirstPersonCharacter.BP_FirstPersonCharacter_C|SetrightHandAvailable (Variables|Default|GetFirst%20PersonCharacter) false)))
  (bind _asplayer_controller (Utilities|Casting|CastToPlayerController (Pawn|GetController (Variables|Default|GetFirst%20PersonCharacter))))
  (Utilities|IsValid (PlayerController|LocalPlayerSubsystems|GetEnhancedInputLocalPlayerSubsystem _asplayer_controller)
    (:Is%20Valid
      (if (Variables|Default|GetLeftHanded)
        (Utilities|FlowControl|Delay 0.1)
        (Input|AddMappingContext (PlayerController|LocalPlayerSubsystems|GetEnhancedInputLocalPlayerSubsystem _asplayer_controller) "/Game/NatsBlueprints/Input/IMC_Spraycan_Left.IMC_Spraycan_Left" 1 "(bIgnoreAllPressedKeysUntilRelease=True,bForceImmediately=False)")
        (else
          (Utilities|FlowControl|Delay 0.1)
          (Input|AddMappingContext (PlayerController|LocalPlayerSubsystems|GetEnhancedInputLocalPlayerSubsystem _asplayer_controller) "/Game/NatsBlueprints/Input/IMC_Spraycan_Right.IMC_Spraycan_Right" 1 "(bIgnoreAllPressedKeysUntilRelease=True,bForceImmediately=False)")))
      (Rendering|Material|SetMaterial 0 (select (> (Variables|Default|GetupgradeAmount%282%29) 0) "/AnimationSharing/AnimSharingGreen.AnimSharingGreen" "/Game/Imports/Viewmodel_Testing/FPV_Spraycan/M_Bugspray_Texture.M_Bugspray_Texture")))))

(event EventUnequip
  (params (SpawnPickup :type Boolean))
  (bind _first_personcharacter (Variables|Default|GetFirst%20PersonCharacter))
  (bind _first_personcharacter_2 (Variables|Default|GetFirst%20PersonCharacter))
  ;[1 1 1] Unequip Logic
  (if SpawnPickup
    (bind _returnvalue (Game|SpawnActorfromClass "/Game/NatsBlueprints/Blueprints/Weapons/One-Handed/Spraycan/BP_Spraycan_Pickup.BP_Spraycan_Pickup_C" (Transformation|GetActorTransform _first_personcharacter) "Undefined" "MultiplyWithRoot" 0 0))
    (Physics|AddForce (Variables|/Game/NatsBlueprints/Blueprints/Weapons/One-Handed/Spraycan/BP_Spraycan_Pickup.BP_Spraycan_Pickup_C|GetSkeletalMesh _returnvalue) (+ (Transformation|GetWorldLocation) (* (Math|Vector|GetForwardVector (Transformation|GetWorldRotation (Variables|/Game/NatsBlueprints/Blueprints/Player/BP_FirstPersonCharacter.BP_FirstPersonCharacter_C|GetFirstPersonCamera (Variables|Default|GetFirst%20PersonCharacter)))) 2.5e+04)) "None" true)
    (Variables|/Game/NatsBlueprints/Blueprints/Weapons/BP_WeaponPickup_Parent.BP_WeaponPickup_Parent_C|SetupgradeAmount%28B%29 _returnvalue (Variables|Default|GetupgradeAmount%282%29)))
  (if (stale EventOnCreate LeftHanded)
    (Variables|/Game/NatsBlueprints/Blueprints/Player/BP_FirstPersonCharacter.BP_FirstPersonCharacter_C|SetbHasLeftHandedSpraycan _first_personcharacter_2 false)
    (else
      (Variables|/Game/NatsBlueprints/Blueprints/Player/BP_FirstPersonCharacter.BP_FirstPersonCharacter_C|SetbHasRightHandedSpraycan _first_personcharacter_2 false)))
  (bind _asplayer_controller (Utilities|Casting|CastToPlayerController (Pawn|GetController _first_personcharacter))
    (:then
      (Utilities|IsValid (PlayerController|LocalPlayerSubsystems|GetEnhancedInputLocalPlayerSubsystem _asplayer_controller)
        (:Is%20Valid
          (if (Variables|Default|GetLeftHanded)
            (Input|RemoveMappingContext (PlayerController|LocalPlayerSubsystems|GetEnhancedInputLocalPlayerSubsystem _asplayer_controller) "/Game/NatsBlueprints/Input/IMC_Spraycan_Left.IMC_Spraycan_Left" "(bIgnoreAllPressedKeysUntilRelease=True,bForceImmediately=False)")
            (else
              (Input|RemoveMappingContext (PlayerController|LocalPlayerSubsystems|GetEnhancedInputLocalPlayerSubsystem _asplayer_controller) "/Game/NatsBlueprints/Input/IMC_Spraycan_Right.IMC_Spraycan_Right" "(bIgnoreAllPressedKeysUntilRelease=True,bForceImmediately=False)"))))
        (:Is%20Not%20Valid
          _)))
    (:CastFailed
      _))
  (Utilities|IsValid (stale Input|EnhancedActionEvents|EnhancedInputActionIA_SprayLeft _returnvalue)
    (:Is%20Valid
      (Actor|DestroyActor (stale Input|EnhancedActionEvents|EnhancedInputActionIA_SprayLeft _returnvalue)))
    (:Is%20Not%20Valid
      _))
  (Utilities|IsValid (stale Input|EnhancedActionEvents|EnhancedInputActionIA_SprayRight _returnvalue)
    (:Is%20Valid
      (Actor|DestroyActor (stale Input|EnhancedActionEvents|EnhancedInputActionIA_SprayRight _returnvalue)))
    (:Is%20Not%20Valid
      _))
  (Utilities|IsValid (stale Input|EnhancedActionEvents|EnhancedInputActionIA_SprayLeft _returnvalue_2)
    (:Is%20Valid
      (Audio|Components|Audio|Stop (stale Input|EnhancedActionEvents|EnhancedInputActionIA_SprayLeft _returnvalue_2)))
    (:Is%20Not%20Valid
      _))
  (Utilities|IsValid (stale Input|EnhancedActionEvents|EnhancedInputActionIA_SprayRight _returnvalue_2)
    (:Is%20Valid
      (Audio|Components|Audio|Stop (stale Input|EnhancedActionEvents|EnhancedInputActionIA_SprayRight _returnvalue_2)))
    (:Is%20Not%20Valid
      _))
  (Components|DestroyComponent))