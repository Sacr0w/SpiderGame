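; Weapon component for a one-handed flyswatter that the first-person character swings at animals from either hand.
; On creation it attaches to the hand socket, sets the character's hand flags and adds that hand's Enhanced Input mapping context.
; Swat input plays a montage whose IMPACT notify sphere-overlaps ahead of the camera, playing hit/miss sounds and damaging animals.
; Unequip optionally throws a spraycan pickup, clears the left-hand flyswatter flag, removes input and destroys itself.
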(event Input|EnhancedActionEvents|EnhancedInputActionIA_Flyswatter_SwatLeft
  (params (ActionValue :type Boolean) (ElapsedSeconds :type Float%20%28double-precision%29) (TriggeredSeconds :type Float%20%28double-precision%29) (InputAction :type Input%20Action%20Object%20Reference :default "/Game/NatsBlueprints/Input/Actions/IA_Flyswatter_SwatLeft.IA_Flyswatter_SwatLeft"))
  (bind _first_personcharacter (Variables|Default|GetFirst%20PersonCharacter))
  (bind _lefthanded (Variables|Default|GetLeftHanded))
  (bind _first_personcharacter_2 (Variables|Default|GetFirst%20PersonCharacter))
  (bind _firstpersonmesh (Variables|/Game/NatsBlueprints/Blueprints/Player/BP_FirstPersonCharacter.BP_FirstPersonCharacter_C|GetFirstPersonMesh _first_personcharacter))
  (bind _firstpersoncamera (Variables|/Game/NatsBlueprints/Blueprints/Player/BP_FirstPersonCharacter.BP_FirstPersonCharacter_C|GetFirstPersonCamera _first_personcharacter_2))
  (:Triggered
    (if _lefthanded
      (if (not (Variables|Default|GetIsAttacking))
        (Variables|Default|SetIsAttacking true)
        (Variables|/Game/NatsBlueprints/Blueprints/Player/BP_FirstPersonCharacter.BP_FirstPersonCharacter_C|SetisAttacking%28Player%29 (Variables|Default|GetFirst%20PersonCharacter) true)
        (if _lefthanded
          (bind _notifyname (Animation|Montage|PlayMontage _firstpersonmesh "/Game/Imports/Viewmodel_Testing/FPV_Limbs/FlyswatterAnims/FlyswatterAttackLEFT_Montage.FlyswatterAttackLEFT_Montage")
            (:OnNotifyBegin
              _))
          (else
            (bind _notifyname_2 (Animation|Montage|PlayMontage _firstpersonmesh "/Game/Imports/Viewmodel_Testing/FPV_Limbs/FlyswatterAnims/FlyswatterAttack_Montage.FlyswatterAttack_Montage")
              (:OnNotifyBegin
                _))))
        (if (or (== _notifyname_2 "IMPACT") (== _notifyname "IMPACT"))
          (bind _outactors (Actor|GetAllActorsOfClass "/Game/NatsBlueprints/Blueprints/Player/BP_FirstPersonCharacter.BP_FirstPersonCharacter_C"))
          (bind (_outactors_2 _returnvalue) (Collision|SphereOverlapActors (+ (Transformation|GetWorldLocation _firstpersoncamera) (* (Math|Vector|GetForwardVector (Transformation|GetWorldRotation _firstpersoncamera)) 1.3e+02)) 8e+01 (Utilities|Array|MakeArray "ObjectTypeQuery3") "/Game/Assets/Animals/Animal_Parent.Animal_Parent_C" _outactors))
          (if _returnvalue
            (Audio|PlaySoundatLocation "/Game/Assets/Audio/Shovel_Hit_01.Shovel_Hit_01" "0, 0, 0" "0, 0, 0" 1.0 1.0 0.0 0 0 0 0)
            (else
              (Audio|PlaySoundatLocation "/Game/Assets/Audio/Shovel_Miss.Shovel_Miss" "0, 0, 0" "0, 0, 0" 1.0 1.0 0.0 0 0 0 0)))
          (for _array_element _outactors_2
            (bind _asanimal_parent (Utilities|Casting|CastToAnimal_Parent _array_element))
            (bind _finaldamage (CallFunction|DamageCalc (Variables|Default|GetbaseDamage)))
            (Default|OnHit _asanimal_parent _finaldamage))
          (else
            (Variables|Default|SetIsAttacking false)
            (Variables|/Game/NatsBlueprints/Blueprints/Player/BP_FirstPersonCharacter.BP_FirstPersonCharacter_C|SetisAttacking%28Player%29 (Variables|Default|GetFirst%20PersonCharacter) false)))))))

(event Input|EnhancedActionEvents|EnhancedInputActionIA_Flyswatter_SwatRight
  (params (ActionValue :type Boolean) (ElapsedSeconds :type Float%20%28double-precision%29) (TriggeredSeconds :type Float%20%28double-precision%29) (InputAction :type Input%20Action%20Object%20Reference :default "/Game/NatsBlueprints/Input/Actions/IA_Flyswatter_SwatRight.IA_Flyswatter_SwatRight"))
  (bind _first_personcharacter (Variables|Default|GetFirst%20PersonCharacter))
  (bind _lefthanded (Variables|Default|GetLeftHanded))
  (bind _first_personcharacter_2 (Variables|Default|GetFirst%20PersonCharacter))
  (bind _firstpersonmesh (Variables|/Game/NatsBlueprints/Blueprints/Player/BP_FirstPersonCharacter.BP_FirstPersonCharacter_C|GetFirstPersonMesh _first_personcharacter))
  (bind _firstpersoncamera (Variables|/Game/NatsBlueprints/Blueprints/Player/BP_FirstPersonCharacter.BP_FirstPersonCharacter_C|GetFirstPersonCamera _first_personcharacter_2))
  (:Triggered
    (if (not _lefthanded)
      (if (not (Variables|Default|GetIsAttacking))
        (Variables|Default|SetIsAttacking true)
        (Variables|/Game/NatsBlueprints/Blueprints/Player/BP_FirstPersonCharacter.BP_FirstPersonCharacter_C|SetisAttacking%28Player%29 (Variables|Default|GetFirst%20PersonCharacter) true)
        (if _lefthanded
          (bind _notifyname (Animation|Montage|PlayMontage _firstpersonmesh "/Game/Imports/Viewmodel_Testing/FPV_Limbs/FlyswatterAnims/FlyswatterAttackLEFT_Montage.FlyswatterAttackLEFT_Montage")
            (:OnNotifyBegin
              _))
          (else
            (bind _notifyname_2 (Animation|Montage|PlayMontage _firstpersonmesh "/Game/Imports/Viewmodel_Testing/FPV_Limbs/FlyswatterAnims/FlyswatterAttack_Montage.FlyswatterAttack_Montage")
              (:OnNotifyBegin
                _))))
        (if (or (== _notifyname_2 "IMPACT") (== _notifyname "IMPACT"))
          (bind _outactors (Actor|GetAllActorsOfClass "/Game/NatsBlueprints/Blueprints/Player/BP_FirstPersonCharacter.BP_FirstPersonCharacter_C"))
          (bind (_outactors_2 _returnvalue) (Collision|SphereOverlapActors (+ (Transformation|GetWorldLocation _firstpersoncamera) (* (Math|Vector|GetForwardVector (Transformation|GetWorldRotation _firstpersoncamera)) 1.3e+02)) 8e+01 (Utilities|Array|MakeArray "ObjectTypeQuery3") "/Game/Assets/Animals/Animal_Parent.Animal_Parent_C" _outactors))
          (if _returnvalue
            (Audio|PlaySoundatLocation "/Game/Assets/Audio/Shovel_Hit_01.Shovel_Hit_01" "0, 0, 0" "0, 0, 0" 1.0 1.0 0.0 0 0 0 0)
            (else
              (Audio|PlaySoundatLocation "/Game/Assets/Audio/Shovel_Miss.Shovel_Miss" "0, 0, 0" "0, 0, 0" 1.0 1.0 0.0 0 0 0 0)))
          (for _array_element _outactors_2
            (bind _asanimal_parent (Utilities|Casting|CastToAnimal_Parent _array_element))
            (bind _finaldamage (CallFunction|DamageCalc (Variables|Default|GetbaseDamage)))
            (Default|OnHit _asanimal_parent _finaldamage))
          (else
            (Variables|Default|SetIsAttacking false)
            (Variables|/Game/NatsBlueprints/Blueprints/Player/BP_FirstPersonCharacter.BP_FirstPersonCharacter_C|SetisAttacking%28Player%29 (Variables|Default|GetFirst%20PersonCharacter) false)))))))

(event EventTick
  (params (DeltaSeconds :type Float%20%28single-precision%29))
  (|CallParentFunction DeltaSeconds) ; This node is disabled and will not be called.\nDrag off pins to build functionality.
)

(event EventOnCreate
  (params (LeftHanded :type Boolean) (SkeletalMeshRef :type Skeletal%20Mesh%20Component%20Object%20Reference))
  ;[1 1 1] Equip Logic
  (bind _output_get (Variables|Default|SetLeftHanded LeftHanded))
  (Variables|Default|SetSkeletalMeshRef SkeletalMeshRef)
  (bind _asbp_first_person_character (Utilities|Casting|CastToBP_FirstPersonCharacter (Components|GetOwner)))
  (bind _output_get_2 (Variables|Default|SetFirst%20PersonCharacter _asbp_first_person_character))
  (Transformation|AttachComponentToComponent (Variables|/Game/NatsBlueprints/Blueprints/Player/BP_FirstPersonCharacter.BP_FirstPersonCharacter_C|GetFirstPersonMesh _output_get_2) (select _output_get "LeftHandedFlyswatterPoint" "RightHandedFlyswatterPoint") "SnapToTarget" "SnapToTarget" "SnapToTarget" true)
  (if (Variables|Default|GetLeftHanded)
    (Variables|/Game/NatsBlueprints/Blueprints/Player/BP_FirstPersonCharacter.BP_FirstPersonCharacter_C|SetbHasLeftHandedFlyswatter (Variables|Default|GetFirst%20PersonCharacter) true)
    (else
      (Variables|/Game/NatsBlueprints/Blueprints/Player/BP_FirstPersonCharacter.BP_FirstPersonCharacter_C|SetbHasRightHandedFlyswatter (Variables|Default|GetFirst%20PersonCharacter) true)))
  (if (Variables|Default|GetLeftHanded)
    (Variables|/Game/NatsBlueprints/Blueprints/Player/BP_FirstPersonCharacter.BP_FirstPersonCharacter_C|SetleftHandAvailable (Variables|Default|GetFirst%20PersonCharacter) false)
    (else
      (Variables|/Game/NatsBlueprints/Blueprints/Player/BP_FirstPersonCharacter.BP_FirstPersonCharacter_C|SetrightHandAvailable (Variables|Default|GetFirst%20PersonCharacter) false)))
  (bind _asplayer_controller (Utilities|Casting|CastToPlayerController (Pawn|GetController (Variables|Default|GetFirst%20PersonCharacter))))
  (Utilities|IsValid (PlayerController|LocalPlayerSubsystems|GetEnhancedInputLocalPlayerSubsystem _asplayer_controller)
    (:Is%20Valid
      (if (Variables|Default|GetLeftHanded)
        (Utilities|FlowControl|Delay 0.05)
        (Input|AddMappingContext (PlayerController|LocalPlayerSubsystems|GetEnhancedInputLocalPlayerSubsystem _asplayer_controller) "/Game/NatsBlueprints/Input/IMC_Flyswatter_Left.IMC_Flyswatter_Left" 1 "(bIgnoreAllPressedKeysUntilRelease=True,bForceImmediately=False)")
        (else
          (Utilities|FlowControl|Delay 0.05)
          (Input|AddMappingContext (PlayerController|LocalPlayerSubsystems|GetEnhancedInputLocalPlayerSubsystem _asplayer_controller) "/Game/NatsBlueprints/Input/IMC_Flyswatter_Right.IMC_Flyswatter_Right" 1 "(bIgnoreAllPressedKeysUntilRelease=True,bForceImmediately=False)"))))))

(event EventUnequip
  (params (SpawnPickup :type Boolean))
  (bind _first_personcharacter (Variables|Default|GetFirst%20PersonCharacter))
  (bind _first_personcharacter_2 (Variables|Default|GetFirst%20PersonCharacter))
  ;[1 1 1] Unequip Logic
  (if SpawnPickup
    (bind _returnvalue (Game|SpawnActorfromClass "/Game/NatsBlueprints/Blueprints/Weapons/One-Handed/Spraycan/BP_Spraycan_Pickup.BP_Spraycan_Pickup_C" (Transformation|GetActorTransform _first_personcharacter) "Undefined" "MultiplyWithRoot" 0 0))
    (Physics|AddForce (Variables|/Game/NatsBlueprints/Blueprints/Weapons/One-Handed/Spraycan/BP_Spraycan_Pickup.BP_Spraycan_Pickup_C|GetSkeletalMesh _returnvalue) (+ (Transformation|GetWorldLocation) (* (Math|Vector|GetForwardVector (Transformation|GetWorldRotation (Variables|/Game/NatsBlueprints/Blueprints/Player/BP_FirstPersonCharacter.BP_FirstPersonCharacter_C|GetFirstPersonCamera (Variables|Default|GetFirst%20PersonCharacter)))) 2.5e+04)) "None" true))
  (if (stale EventOnCreate LeftHanded)
    (Variables|/Game/NatsBlueprints/Blueprints/Player/BP_FirstPersonCharacter.BP_FirstPersonCharacter_C|SetbHasLeftHandedFlyswatter _first_personcharacter_2 false)
    (else
      (Variables|/Game/NatsBlueprints/Blueprints/Player/BP_FirstPersonCharacter.BP_FirstPersonCharacter_C|SetbHasLeftHandedFlyswatter _first_personcharacter_2 false)))
  (bind _asplayer_controller (Utilities|Casting|CastToPlayerController (Pawn|GetController _first_personcharacter))
    (:then
      (Utilities|IsValid (PlayerController|LocalPlayerSubsystems|GetEnhancedInputLocalPlayerSubsystem _asplayer_controller)
        (:Is%20Valid
          (if (Variables|Default|GetLeftHanded)
            (Input|RemoveMappingContext (PlayerController|LocalPlayerSubsystems|GetEnhancedInputLocalPlayerSubsystem _asplayer_controller) "/Game/NatsBlueprints/Input/IMC_Flyswatter_Left.IMC_Flyswatter_Left" "(bIgnoreAllPressedKeysUntilRelease=True,bForceImmediately=False)")
            (else
              (Input|RemoveMappingContext (PlayerController|LocalPlayerSubsystems|GetEnhancedInputLocalPlayerSubsystem _asplayer_controller) "/Game/NatsBlueprints/Input/IMC_Flyswatter_Right.IMC_Flyswatter_Right" "(bIgnoreAllPressedKeysUntilRelease=True,bForceImmediately=False)"))))
        (:Is%20Not%20Valid
          _)))
    (:CastFailed
      _))
  (Components|DestroyComponent))