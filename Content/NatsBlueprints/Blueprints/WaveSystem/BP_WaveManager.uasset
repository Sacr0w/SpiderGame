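; Wave manager that starts a spider enemy wave shortly after BeginPlay, sized by wave count.
; A delayed loop sphere-checks four spawn points, drops those near the first-person player and picks one at random.
; SpawnEnemyGroup spawns the whole remaining count there, but only when it is eight or fewer.
; Once spawning ends, it polls until no Animal_Parent actors remain, then clears the wave flag without starting another.
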(event Custom|StartWave
  ;[1 1 1] InitialiseWaveLogic
  (if (not (Variables|Default|GetWaveActive%28Presence%29))
    (bind _output_get (Variables|Default|SetWaveCount (+ (Variables|Default|GetWaveCount) 1)))
    (Variables|Default|SetEnemiesToSpawn (* _output_get 5))
    (Variables|Default|SetWaveActive%28Presence%29 true)
    (Variables|Default|SetWaveActive%28Spawning%29 true)
    ;[1 1 1] WaveLoopLogic
    (if (Variables|Default|GetWaveActive%28Spawning%29) :!label _label
      (bind _outactors (Actor|GetAllActorsOfClass "/Game/Assets/Animals/Animal_Parent.Animal_Parent_C"))
      (Utilities|FlowControl|Delay (select (<= (Utilities|Array|Length _outactors) 0) 0.0 (Math|Conversions|ToFloat(Integer) (Math|Random|RandomIntegerinRange 5 15))))
      (Variables|Default|SetActiveSpawnArray (Utilities|Array|MakeArray (Variables|Default|GetEnemySpawn1) (Variables|Default|GetEnemySpawn2) (Variables|Default|GetEnemySpawn3) (Variables|Default|GetEnemySpawn4)))
      (Utilities|FlowControl|Sequence
        (:then_0
          (Variables|Default|SetSpawnToCompare (Variables|Default|GetEnemySpawn1)))
        (:then_1
          (Variables|Default|SetSpawnToCompare (Variables|Default|GetEnemySpawn2)))
        (:then_2
          (Variables|Default|SetSpawnToCompare (Variables|Default|GetEnemySpawn3)))
        (:then_3
          (Variables|Default|SetSpawnToCompare (Variables|Default|GetEnemySpawn4)))
        (:then_4
          (if (Utilities|Array|IsNotEmpty (Variables|Default|GetActiveSpawnArray))
            (CallFunction|SpawnEnemyGroup (Utilities|Array|Get(acopy) (Variables|Default|GetActiveSpawnArray) (Math|Random|RandomIntegerinRange 0 (Utilities|Array|Length (Variables|Default|GetActiveSpawnArray)))))
            (Utilities|FlowControl|Delay 5.0)
            (if (<= (Variables|Default|GetEnemiesToSpawn) 0)
              (Variables|Default|SetWaveActive%28Spawning%29 false)
              (goto _label)
              (else
                (goto _label)))
            (else
              (goto _label)))))
      (bind _returnvalue (Collision|SphereOverlapActors (Transformation|GetWorldLocation (Variables|Default|GetSpawnToCompare)) 3e+02 (Utilities|Array|MakeArray "ObjectTypeQuery3") "/Game/NatsBlueprints/Blueprints/Player/BP_FirstPersonCharacter.BP_FirstPersonCharacter_C"))
      (if _returnvalue
        ;[1 1 1] PlayerIsNearSpawn
        (if (== (Utilities|GetObjectName (Variables|Default|GetSpawnToCompare)) "EnemySpawn1")
          (Variables|Default|SetSpawn1Active? false)
          (Utilities|Array|RemoveItem (Variables|Default|GetActiveSpawnArray) (Variables|Default|GetEnemySpawn1))
          (Development|PrintText "SpawnInvalid" :!label _label_2)
          (elif (== (Utilities|GetObjectName (Variables|Default|GetSpawnToCompare)) "EnemySpawn2")
            (Variables|Default|SetSpawn2Active? false)
            (Utilities|Array|RemoveItem (Variables|Default|GetActiveSpawnArray) (Variables|Default|GetEnemySpawn2))
            (goto _label_2)
            (elif (== (Utilities|GetObjectName (Variables|Default|GetSpawnToCompare)) "EnemySpawn3")
              (Variables|Default|SetSpawn3Active? false)
              (Utilities|Array|RemoveItem (Variables|Default|GetActiveSpawnArray) (Variables|Default|GetEnemySpawn3))
              (goto _label_2)
              (elif (== (Utilities|GetObjectName (Variables|Default|GetSpawnToCompare)) "EnemySpawn4")
                (Variables|Default|SetSpawn4Active? false)
                (Utilities|Array|RemoveItem (Variables|Default|GetActiveSpawnArray) (Variables|Default|GetEnemySpawn4))
                (goto _label_2)))))
        (else
          ;[1 1 1] PlayerNOTNearSpawn
          (if (== (Utilities|GetObjectName (Variables|Default|GetSpawnToCompare)) "EnemySpawn1")
            (Variables|Default|SetSpawn1Active? true)
            (Development|PrintText "SpawnValid" :!label _label_3)
            (elif (== (Utilities|GetObjectName (Variables|Default|GetSpawnToCompare)) "EnemySpawn2")
              (Variables|Default|SetSpawn2Active? true)
              (goto _label_3)
              (elif (== (Utilities|GetObjectName (Variables|Default|GetSpawnToCompare)) "EnemySpawn3")
                (Variables|Default|SetSpawn3Active? true)
                (goto _label_3)
                (elif (== (Utilities|GetObjectName (Variables|Default|GetSpawnToCompare)) "EnemySpawn4")
                  (Variables|Default|SetSpawn4Active? true)
                  (goto _label_3)))))))
      (else
        (bind _outactors_2 (Actor|GetAllActorsOfClass "/Game/Assets/Animals/Animal_Parent.Animal_Parent_C" :!label _label_4))
        (if (<= (Utilities|Array|Length _outactors_2) 0)
          (Variables|Default|SetWaveActive%28Presence%29 false)
          (else
            (Utilities|FlowControl|Delay 3.0)
            (goto _label_4)))))))

(event Custom|SpawnEnemyGroup
  (params (SpawnPoint :type Static%20Mesh%20Component%20Object%20Reference))
  (Utilities|IsValid SpawnPoint
    (:Is%20Valid
      (Variables|Default|SetSpawn%20Point SpawnPoint)
      (if (> (Variables|Default|GetEnemiesToSpawn) 0)
        (if (<= (Variables|Default|GetEnemiesToSpawn) 8)
          (if (> (Variables|Default|GetEnemiesToSpawn) 0) :!label _label
            (Game|SpawnActorfromClass "/Game/Assets/Animals/Spider/BP_AI_Spider.BP_AI_Spider_C" (Transformation|GetWorldTransform (Variables|Default|GetSpawn%20Point)) "Undefined" "MultiplyWithRoot" 0 0)
            (Variables|Default|SetEnemiesToSpawn (- (Variables|Default|GetEnemiesToSpawn) 1))
            (goto _label)))))))

(event EventBeginPlay
  (Utilities|FlowControl|Delay 2.0)
  (CallFunction|StartWave))

(event Collision|EventActorBeginOverlap
  (params (OtherActor :type Actor%20Object%20Reference)))

(event EventTick
  (params (DeltaSeconds :type Float%20%28single-precision%29)))

(fn ConstructionScript)