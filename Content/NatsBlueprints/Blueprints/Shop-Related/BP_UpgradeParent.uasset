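; Base actor for shop upgrades, showing a spinning cube with an info widget and supporting purchase with Spidercoins.
; InitialiseInfo fills the widget and sets the cost from a data table row chosen by InfoRow.
; Repeated Highlight calls keep the player-facing widget visible through a short retriggerable delay.
; OnPurchase deducts affordable costs then fires the empty OnPickup hook, which player overlap also triggers at no charge.
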(event Custom|OnPickup)

(event Custom|Highlight
  (Variables|Default|SetHighlighted true)
  (Utilities|FlowControl|RetriggerableDelay 0.05)
  (Variables|Default|SetHighlighted false))

(event Custom|OnPurchase
  (bind _playerref (Variables|Default|GetPlayerRef))
  (if (>= (Variables|/Game/NatsBlueprints/Blueprints/Player/BP_FirstPersonCharacter.BP_FirstPersonCharacter_C|GetSpidercoinCount _playerref) (Variables|Default|GetObjectCost))
    (Variables|/Game/NatsBlueprints/Blueprints/Player/BP_FirstPersonCharacter.BP_FirstPersonCharacter_C|SetSpidercoinCount _playerref (- (Variables|/Game/NatsBlueprints/Blueprints/Player/BP_FirstPersonCharacter.BP_FirstPersonCharacter_C|GetSpidercoinCount _playerref) (Variables|Default|GetObjectCost)))
    (CallFunction|OnPickup)))

(event EventBeginPlay
  (bind _asbp_first_person_character (Utilities|Casting|CastToBP_FirstPersonCharacter (Game|GetPlayerCharacter 0)))
  (Variables|Default|SetPlayerRef _asbp_first_person_character)
  (CallFunction|InitialiseInfo))

(event Collision|EventActorBeginOverlap
  (params (OtherActor :type Actor%20Object%20Reference))
  (Utilities|Casting|CastToBP_FirstPersonCharacter OtherActor)
  (CallFunction|OnPickup))

(event EventTick
  (params (DeltaSeconds :type Float%20%28single-precision%29))
  (bind _cube (Variables|Default|GetCube))
  (bind _upgradeinfo (Variables|Default|GetUpgradeInfo))
  (Transformation|SetWorldRotation _cube (Math|Rotator|MakeRotator 0.0 0.0 (+ (.yaw (Transformation|GetWorldRotation _cube)) 1.0)) false false)
  (if (Variables|Default|GetHighlighted)
    (Rendering|SetVisibility _upgradeinfo true false)
    (else
      (Rendering|SetVisibility _upgradeinfo false false)))
  (if (Variables|Default|GetHighlighted)
    (Transformation|SetWorldLocationAndRotation (Variables|Default|GetUpgradeInfo) (+ (Transformation|GetActorLocation) (Variables|Default|GetInfoScreenOffset)) (Math|Rotator|FindLookatRotation (+ (Transformation|GetActorLocation) (Variables|Default|GetInfoScreenOffset)) (.OutLocation (Actor|GetActorEyesViewPoint (Game|GetPlayerCharacter 0)))) false true)))

(fn ConstructionScript)

(fn InitialiseInfo
  (bind _aswb_upgrade_info (Utilities|Casting|CastToWB_UpgradeInfo (UserInterface|GetUserWidgetObject (Variables|Default|GetUpgradeInfo))))
  (LocalVariables|SetUpgradeInfoRef _aswb_upgrade_info)
  (bind _returnvalue (Class|DataTableFunctionLibrary|DoesDataTableRowExist "/Game/NatsBlueprints/Blueprints/Shop-Related/UpgradeInfoTable.UpgradeInfoTable" (Variables|Default|GetInfoRow)))
  (if _returnvalue
    (bind _returnvalue_2 (Utilities|GetDataTableRow "/Game/NatsBlueprints/Blueprints/Shop-Related/UpgradeInfoTable.UpgradeInfoTable" (Variables|Default|GetInfoRow))
      (:then
        (LocalVariables|SetRowRef _returnvalue_2)
        (Utilities|FlowControl|Sequence
          (:then_0
            (Variables|/Game/NatsBlueprints/Blueprints/Shop-Related/WB_UpgradeInfo.WB_UpgradeInfo_C|SetName (LocalVariables|GetUpgradeInfoRef) (.Name (Utilities|Struct|BreakS_UpgradeStructure (LocalVariables|GetRowRef)))))
          (:then_1
            (Variables|/Game/NatsBlueprints/Blueprints/Shop-Related/WB_UpgradeInfo.WB_UpgradeInfo_C|SetFlavourText (LocalVariables|GetUpgradeInfoRef) (.FlavourText (Utilities|Struct|BreakS_UpgradeStructure (LocalVariables|GetRowRef)))))
          (:then_2
            (Variables|/Game/NatsBlueprints/Blueprints/Shop-Related/WB_UpgradeInfo.WB_UpgradeInfo_C|SetDescription (LocalVariables|GetUpgradeInfoRef) (.Description (Utilities|Struct|BreakS_UpgradeStructure (LocalVariables|GetRowRef)))))
          (:then_3
            (Variables|/Game/NatsBlueprints/Blueprints/Shop-Related/WB_UpgradeInfo.WB_UpgradeInfo_C|SetColour (LocalVariables|GetUpgradeInfoRef) (.Colour (Utilities|Struct|BreakS_UpgradeStructure (LocalVariables|GetRowRef)))))
          (:then_4
            (bind _output_get (Variables|/Game/NatsBlueprints/Blueprints/Shop-Related/WB_UpgradeInfo.WB_UpgradeInfo_C|SetCost (LocalVariables|GetUpgradeInfoRef) (.Cost (Utilities|Struct|BreakS_UpgradeStructure (LocalVariables|GetRowRef)))))
            (Variables|Default|SetObjectCost _output_get)))))))