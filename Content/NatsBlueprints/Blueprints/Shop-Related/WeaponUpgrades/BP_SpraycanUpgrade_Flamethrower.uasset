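; Shop upgrade pickup that upgrades the player's spraycan into a flamethrower.
; On pickup, it casts the weapon in the left or right hand to the spraycan component and calls its upgrade.
; It then spawns a flamethrower pickup at a fixed elevated location, makes the player pick it up after a brief delay, and destroys itself.
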(event EventBeginPlay
  (|CallParentFunction) ; This node is disabled and will not be called.\nDrag off pins to build functionality.
)

(event Collision|EventActorBeginOverlap
  (params (OtherActor :type Actor%20Object%20Reference))
  (|CallParentFunction OtherActor) ; This node is disabled and will not be called.\nDrag off pins to build functionality.
)

(event EventTick
  (params (DeltaSeconds :type Float%20%28single-precision%29))
  (|CallParentFunction DeltaSeconds) ; This node is disabled and will not be called.\nDrag off pins to build functionality.
)

(event EventOnPickup
  (params (LeftHanded :type Boolean))
  (bind _playerref (Variables|Default|GetPlayerRef))
  (if LeftHanded
    (bind _asbp_spraycan_component (Utilities|Casting|CastToBP_Spraycan_Component (Variables|/Game/NatsBlueprints/Blueprints/Player/BP_FirstPersonCharacter.BP_FirstPersonCharacter_C|GetleftWeaponEquipped _playerref)))
    (Default|OnUpgrade _asbp_spraycan_component true)
    (else
      (bind _asbp_spraycan_component_2 (Utilities|Casting|CastToBP_Spraycan_Component (Variables|/Game/NatsBlueprints/Blueprints/Player/BP_FirstPersonCharacter.BP_FirstPersonCharacter_C|GetrightWeaponEquipped _playerref)))
      (Default|OnUpgrade _asbp_spraycan_component_2 true)))
  (bind _returnvalue (Game|SpawnActorfromClass "/Game/NatsBlueprints/Blueprints/Weapons/Two-Handed/Spraycan_Lighter/BP_Flamethrower_Pickup.BP_Flamethrower_Pickup_C" (Math|Transform|MakeTransform "0.000000,0.000000,1000.000000") "Undefined" "MultiplyWithRoot" 0 0))
  (Utilities|FlowControl|Delay 0.05)
  (Default|Pickup _returnvalue (Variables|Default|GetPlayerRef) false false false)
  (Actor|DestroyActor))

(fn ConstructionScript
  (|CallParentFunction))