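; Shop weapon-upgrade pickup actor for the Weedkiller upgrade of the spraycan.
; On pickup, it takes the player's left or right equipped weapon according to the hand flag and casts it to the spraycan component.
; It calls OnUpgrade on that component with a false flag, then destroys itself.
; If that hand holds no spraycan, the cast fails and the pickup stays.
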(event EventBeginPlay
  (|CallParentFunction) ; This node is disabled and will not be called.\nDrag off pins to build functionality.
)

(event Collision|EventActorBeginOverlap
  (params (OtherActor :type Actor%20Object%20Reference))
  (|CallParentFunction OtherActor) ; This node is disabled and will not be called.\nDrag off pins to build functionality.
)

(event EventTick
  (params (DeltaSeconds :type Float%20%28single-precision%29))
  (|CallParentFunction DeltaSeconds) ; This node is disabled and will not be called.\nDrag off pins to build functionality.
)

(event EventOnPickup
  (params (LeftHanded :type Boolean))
  (bind _playerref (Variables|Default|GetPlayerRef))
  (if LeftHanded
    (bind _asbp_spraycan_component (Utilities|Casting|CastToBP_Spraycan_Component (Variables|/Game/NatsBlueprints/Blueprints/Player/BP_FirstPersonCharacter.BP_FirstPersonCharacter_C|GetleftWeaponEquipped _playerref)))
    (Default|OnUpgrade _asbp_spraycan_component false)
    (else
      (bind _asbp_spraycan_component_2 (Utilities|Casting|CastToBP_Spraycan_Component (Variables|/Game/NatsBlueprints/Blueprints/Player/BP_FirstPersonCharacter.BP_FirstPersonCharacter_C|GetrightWeaponEquipped _playerref)))
      (Default|OnUpgrade _asbp_spraycan_component_2 false)))
  (Actor|DestroyActor))

(fn ConstructionScript
  (|CallParentFunction))