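; BP_ShovelUpgrade_Rake is a weapon upgrade pickup, filed with the shop's upgrades, that upgrades the player's shovel.
; On pickup it casts the player's equipped two-handed weapon to BP_Shovel_Component, calls OnUpgrade with true, then destroys itself.
; If the cast fails, nothing happens and the actor remains.
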(event EventBeginPlay
  (|CallParentFunction) ; This node is disabled and will not be called.\nDrag off pins to build functionality.
)

(event Collision|EventActorBeginOverlap
  (params (OtherActor :type Actor%20Object%20Reference))
  (|CallParentFunction OtherActor) ; This node is disabled and will not be called.\nDrag off pins to build functionality.
)

(event EventTick
  (params (DeltaSeconds :type Float%20%28single-precision%29))
  (|CallParentFunction DeltaSeconds) ; This node is disabled and will not be called.\nDrag off pins to build functionality.
)

(event EventOnPickup
  (bind _asbp_shovel_component (Utilities|Casting|CastToBP_Shovel_Component (Variables|/Game/NatsBlueprints/Blueprints/Player/BP_FirstPersonCharacter.BP_FirstPersonCharacter_C|GettwoHandedWeaponEquipped (Variables|Default|GetPlayerRef))))
  (Default|OnUpgrade _asbp_shovel_component true)
  (Actor|DestroyActor))

(fn ConstructionScript
  (|CallParentFunction))