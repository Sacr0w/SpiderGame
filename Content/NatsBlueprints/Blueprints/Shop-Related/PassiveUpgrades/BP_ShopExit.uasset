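; BP_ShopExit is a shop pickup that ends the shop phase and resumes combat waves.
; On pickup, it finds BP_MainShop to clean up the shop, then finds BP_WaveManager to reset the countdown to the next shop and start a wave.
; It destroys itself afterward.
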(event EventBeginPlay
  (|CallParentFunction) ; This node is disabled and will not be called.\nDrag off pins to build functionality.
)

(event Collision|EventActorBeginOverlap
  (params (OtherActor :type Actor%20Object%20Reference))
  (|CallParentFunction OtherActor) ; This node is disabled and will not be called.\nDrag off pins to build functionality.
)

(event EventTick
  (params (DeltaSeconds :type Float%20%28single-precision%29))
  (|CallParentFunction DeltaSeconds) ; This node is disabled and will not be called.\nDrag off pins to build functionality.
)

(event EventOnPickup
  (bind _returnvalue (Actor|GetActorOfClass "/Game/NatsBlueprints/Blueprints/Shop-Related/BP_MainShop.BP_MainShop_C"))
  (Default|CleanupShop _returnvalue)
  (bind _returnvalue_2 (Actor|GetActorOfClass "/Game/NatsBlueprints/Blueprints/WaveSystem/BP_WaveManager.BP_WaveManager_C"))
  (Variables|/Game/NatsBlueprints/Blueprints/WaveSystem/BP_WaveManager.BP_WaveManager_C|SetWavesUntilShop _returnvalue_2 5)
  (Default|StartWave _returnvalue_2)
  (Actor|DestroyActor))

(fn ConstructionScript
  (|CallParentFunction))