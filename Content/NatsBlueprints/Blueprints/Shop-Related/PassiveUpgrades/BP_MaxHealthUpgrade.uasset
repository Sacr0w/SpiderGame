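; BP_MaxHealthUpgrade is a passive upgrade pickup, filed under shop content, that raises the player's maximum health and heals them.
; On pickup it calls the player's HealFunc twice: first with a flat amount that increases max HP, then with a fraction of max HP as healing.
; The actor then destroys itself, and its other events are disabled stubs.
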(event EventBeginPlay
  (|CallParentFunction) ; This node is disabled and will not be called.\nDrag off pins to build functionality.
)

(event Collision|EventActorBeginOverlap
  (params (OtherActor :type Actor%20Object%20Reference))
  (|CallParentFunction OtherActor) ; This node is disabled and will not be called.\nDrag off pins to build functionality.
)

(event EventTick
  (params (DeltaSeconds :type Float%20%28single-precision%29))
  (|CallParentFunction DeltaSeconds) ; This node is disabled and will not be called.\nDrag off pins to build functionality.
)

(event EventOnPickup
  (params (LeftHanded :type Boolean))
  (bind _playerref (Variables|Default|GetPlayerRef))
  (Default|HealFunc _playerref 5e+01 true false)
  (Default|HealFunc _playerref 0.5 false true)
  (Actor|DestroyActor))

(fn ConstructionScript
  (|CallParentFunction))