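; BP_DamageUpgrade is a shop passive upgrade that permanently boosts the player's damage.
; On pickup it adds a fixed increment to the player's base damage percent through PlayerRef, then destroys itself.
; All other events are disabled stubs, and the construction script only calls its parent.
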(event EventBeginPlay
  (|CallParentFunction) ; This node is disabled and will not be called.\nDrag off pins to build functionality.
)

(event Collision|EventActorBeginOverlap
  (params (OtherActor :type Actor%20Object%20Reference))
  (|CallParentFunction OtherActor) ; This node is disabled and will not be called.\nDrag off pins to build functionality.
)

(event EventTick
  (params (DeltaSeconds :type Float%20%28single-precision%29))
  (|CallParentFunction DeltaSeconds) ; This node is disabled and will not be called.\nDrag off pins to build functionality.
)

(event EventOnPickup
  (bind _playerref (Variables|Default|GetPlayerRef))
  (Variables|/Game/NatsBlueprints/Blueprints/Player/BP_FirstPersonCharacter.BP_FirstPersonCharacter_C|SetPlayerBaseDamagePercent _playerref (+ (Variables|/Game/NatsBlueprints/Blueprints/Player/BP_FirstPersonCharacter.BP_FirstPersonCharacter_C|GetPlayerBaseDamagePercent _playerref) 0.2))
  (Actor|DestroyActor))

(fn ConstructionScript
  (|CallParentFunction))