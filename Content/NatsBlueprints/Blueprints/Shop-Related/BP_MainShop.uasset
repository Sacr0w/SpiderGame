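; BP_MainShop is a shop actor that stocks five random upgrades and an exit when play begins.
; SpawnUpgrade fills each slot component with either a max health or damage upgrade at even odds, storing each actor in a numbered variable.
; A BP_ShopExit spawns at the Button component without its reference being stored.
; CleanupShop destroys the five stored upgrades and the shop itself, but not the spawned exit.
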(event Custom|CleanupShop
  (Actor|DestroyActor (Variables|Default|GetUpgrade1))
  (Actor|DestroyActor (Variables|Default|GetUpgrade2))
  (Actor|DestroyActor (Variables|Default|GetUpgrade3))
  (Actor|DestroyActor (Variables|Default|GetUpgrade4))
  (Actor|DestroyActor (Variables|Default|GetUpgrade5))
  (Actor|DestroyActor))

(event Custom|SpawnUpgrade
  (params (SpawnTransform :type Transform) (Number :type Integer))
  (if (== (Math|Random|RandomIntegerinRange 0 1) 0)
    (Variables|Default|SetClass "/Game/NatsBlueprints/Blueprints/Shop-Related/PassiveUpgrades/BP_MaxHealthUpgrade.BP_MaxHealthUpgrade_C")
    (else
      (Variables|Default|SetClass "/Game/NatsBlueprints/Blueprints/Shop-Related/PassiveUpgrades/BP_DamageUpgrade.BP_DamageUpgrade_C")))
  (bind _returnvalue (Game|SpawnActorfromClass (Variables|Default|GetClass) (Math|Transform|MakeTransform (.location SpawnTransform) (.rotation SpawnTransform) "1.000000,1.000000,1.000000") "Undefined" "MultiplyWithRoot" 0 0))
  (if (== Number 1)
    (Variables|Default|SetUpgrade1 _returnvalue)
    (elif (== Number 2)
      (Variables|Default|SetUpgrade2 _returnvalue)
      (elif (== Number 3)
        (Variables|Default|SetUpgrade3 _returnvalue)
        (elif (== Number 4)
          (Variables|Default|SetUpgrade4 _returnvalue)
          (elif (== Number 5)
            (Variables|Default|SetUpgrade5 _returnvalue)))))))

(event EventBeginPlay
  (bind _button (Variables|Default|GetButton))
  (bind _returnvalue (Transformation|GetWorldTransform _button))
  (Utilities|FlowControl|Sequence
    (:then_0
      (CallFunction|SpawnUpgrade (Transformation|GetWorldTransform (Variables|Default|GetSlot1)) 1))
    (:then_1
      (CallFunction|SpawnUpgrade (Transformation|GetWorldTransform (Variables|Default|GetSlot2)) 2))
    (:then_2
      (CallFunction|SpawnUpgrade (Transformation|GetWorldTransform (Variables|Default|GetSlot3)) 3))
    (:then_3
      (CallFunction|SpawnUpgrade (Transformation|GetWorldTransform (Variables|Default|GetSlot4)) 4))
    (:then_4
      (CallFunction|SpawnUpgrade (Transformation|GetWorldTransform (Variables|Default|GetSlot5)) 5))
    (:then_5
      (Game|SpawnActorfromClass "/Game/NatsBlueprints/Blueprints/Shop-Related/PassiveUpgrades/BP_ShopExit.BP_ShopExit_C" (Math|Transform|MakeTransform (.location _returnvalue) (.rotation _returnvalue) "1.000000,1.000000,1.000000") "Undefined" "MultiplyWithRoot" 0 0))))

(event Collision|EventActorBeginOverlap
  (params (OtherActor :type Actor%20Object%20Reference)))

(event EventTick
  (params (DeltaSeconds :type Float%20%28single-precision%29)))

(fn ConstructionScript)