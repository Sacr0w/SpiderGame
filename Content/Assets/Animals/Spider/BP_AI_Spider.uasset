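; Spider enemy AI that roams, chases the first-person player and bites at close range.
; Pawn sensing starts an AI MoveTo chase, and a one-second timer issues random roam moves when the player hasn't been seen since its last check.
; Delay-throttled Tick destroys the spider at zero HP or checks a small overlap sphere, triggering an attack montage that deals damage after a short delay through a wider sphere.
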(event OnSeePawn(PawnSensing)
  (params (Pawn :type Pawn%20Object%20Reference))
  ;[1 0 0] "Stop! You violated the law! Pay the court a fine or serve your sentence. Your stolen goods ar..."
  (Variables|Default|SetfoundPlayer true)
  (Variables|Default|SetisRoaming false)
  (if (not (Variables|Default|GetisAttacking))
    (CallFunction|FollowPlayer)))

(event Custom|FollowPlayer
  ;[1 0 0] "Stop! You violated the law! Pay the court a fine or serve your sentence. Your stolen goods ar..."
  (AI|AIMoveTo self "0, 0, 0" (Variables|Default|GetCharRef) 5.0 false))

(event Custom|RandomRoam
  ;[0.04076 0.9602 1] RandomRoamLogic
  (AI|AIMoveTo self (.RandomLocation (AI|Navigation|GetRandomReachablePointinRadius (Transformation|GetActorLocation) 5e+02 0 0)) 0 5.0 false))

(event Custom|CheckIsChasing
  ;[0.04076 0.9602 1] RandomRoamLogic
  (if (not (Variables|Default|GetisAttacking))
    (if (Variables|Default|GetfoundPlayer)
      (Variables|Default|SetfoundPlayer false)
      (elif (not (Variables|Default|GetisRoaming))
        (CallFunction|RandomRoam)))))

(event EventBeginPlay
  (bind _returnvalue (Actor|GetActorOfClass "/Game/NatsBlueprints/Blueprints/BP_FirstPersonCharacter.BP_FirstPersonCharacter_C"))
  (Variables|Default|SetCharRef _returnvalue)
  (Utilities|Time|SetTimerbyEvent (delegate Custom|CheckIsChasing) 1.0 true))

(event EventTick
  (params (DeltaSeconds :type Float%20%28single-precision%29))
  ;[0.08416 0.1432 1] ded :<
  (if (<= (Variables|Default|GetcurrHP) 0.0)
    (Actor|DestroyActor)
    (else
      (Utilities|FlowControl|Delay 0.1)
      (if (not (Variables|Default|GetisAttacking))
        ;[1 0.3015 0.0599] Point Blank
        (bind _outactors (Collision|SphereOverlapActors (Transformation|GetActorLocation) 9e+01 (Utilities|Array|MakeArray "ObjectTypeQuery3") 0))
        (bind _array_element (Utilities|Array|ForEachLoopwithBreak _outactors :!label _label)
          (:LoopBody
            (Utilities|Casting|CastToBP_FirstPersonCharacter _array_element)
            (Variables|Default|SetisAttacking true)
            (goto _label Break))
          (:Completed
            (if (Variables|Default|GetisAttacking)
              (Class|NavMovementComponent|StopActiveMovement (Variables|Character|GetCharacterMovement))
              (Animation|Montage|PlayMontage (Variables|Character|GetMesh) "/Game/Assets/Animals/Spider/Spider_Attack_Montage.Spider_Attack_Montage"
                (:then
                  (Utilities|FlowControl|Delay 0.4)
                  (bind _outactors_2 (Collision|SphereOverlapActors (Transformation|GetActorLocation) 1.2e+02 (Utilities|Array|MakeArray "ObjectTypeQuery3") 0))
                  (bind _array_element_2 (Utilities|Array|ForEachLoopwithBreak _outactors_2 :!label _label_2)
                    (:LoopBody
                      (bind _asbp_first_person_character (Utilities|Casting|CastToBP_FirstPersonCharacter _array_element_2))
                      (Development|PrintString "OW")
                      (Variables|/Game/NatsBlueprints/Blueprints/BP_FirstPersonCharacter.BP_FirstPersonCharacter_C|SetHP _asbp_first_person_character (- (Variables|/Game/NatsBlueprints/Blueprints/BP_FirstPersonCharacter.BP_FirstPersonCharacter_C|GetHP _asbp_first_person_character) 1e+01))
                      (goto _label_2 Break))))
                (:OnCompleted
                  _)
                (:OnInterrupted
                  _))
              (Variables|Default|SetisAttacking false))))))))

(fn ConstructionScript)