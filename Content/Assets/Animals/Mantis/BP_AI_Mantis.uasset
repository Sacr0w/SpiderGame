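; Mantis enemy AI that roams randomly until it sees a pawn, then speeds up and chases the first-person player.
; A looping timer drives movement, aiming at random sideways offsets from the player's camera until close, then straight at the player.
; Tick runs a proximity check that triggers a melee montage, whose notify applies damage through a second sphere overlap.
; A camera-facing health bar, using Spider-named assets, appears briefly when hit.
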(event OnSeePawn(PawnSensing)
  (params (Pawn :type Pawn%20Object%20Reference))
  ;[1 0 0] "Stop! You violated the law! Pay the court a fine or serve your sentence. Your stolen goods ar..."
  (if (not (Variables|Default|GetfoundPlayer))
    (Variables|Default|SetfoundPlayer true)
    (Variables|Default|SetisRoaming false)
    (Utilities|Time|SetTimerbyEvent (delegate Custom|CheckIsChasing) 0.2 true)
    (Variables|Default|SetbaseSpeed 6e+02)
    (Variables|Default|Setspeed 6e+02)))

(event Custom|FollowPlayer
  (bind _self self)
  (bind _charref (Variables|Default|GetCharRef))
  (bind _firstpersoncamera (Variables|/Game/NatsBlueprints/Blueprints/Player/BP_FirstPersonCharacter.BP_FirstPersonCharacter_C|GetFirstPersonCamera _charref))
  (bind _returnvalue (Transformation|GetWorldRotation _firstpersoncamera))
  (bind _returnvalue_2 (Math|Vector|GetRightVector _returnvalue))
  ;[1 0 0] "Stop! You violated the law! Pay the court a fine or serve your sentence. Your stolen goods ar..."
  (bind _returnvalue_3 (Collision|SphereOverlapActors (Transformation|GetActorLocation) 2e+02 (Utilities|Array|MakeArray "ObjectTypeQuery3") "/Game/NatsBlueprints/Blueprints/Player/BP_FirstPersonCharacter.BP_FirstPersonCharacter_C"))
  (if _returnvalue_3
    (AI|AIMoveTo _self "0, 0, 0" (Variables|Default|GetCharRef) 5.0 false)
    (else
      (AI|AIMoveTo _self (+ (Transformation|GetWorldLocation _firstpersoncamera) (* (Math|Vector|MakeVector (.x _returnvalue_2) (.y _returnvalue_2) 0.0) (Math|Random|RandomFloatinRange -4e+02 4e+02))) 0 5.0 false))))

(event Custom|RandomRoam
  ;[0.7232 0.2868 1] RandomRoamLogic
  (AI|AIMoveTo self (.RandomLocation (AI|Navigation|GetRandomReachablePointinRadius (Transformation|GetActorLocation) 5e+02 0 0)) 0 5.0 false))

(event Custom|CheckIsChasing
  ;[0.7232 0.2868 1] RandomRoamLogic
  (if (not (Variables|Default|GetisAttacking))
    (if (Variables|Default|GetfoundPlayer)
      (CallFunction|FollowPlayer)
      (elif (not (Variables|Default|GetisRoaming))
        (CallFunction|RandomRoam)))))

(event EventOnHit
  (params (DamageTaken :type Float%20%28double-precision%29))
  ;[0.04365 1 0.09143] ouchies Logic
  (Variables|Default|SetcurrHP (- (Variables|Default|GetcurrHP) (Utilities|DamageResistCalc DamageTaken)))
  (Rendering|SetVisibility (Variables|Default|GetSpiderHP) true false)
  (Utilities|FlowControl|RetriggerableDelay 3.0)
  (Rendering|SetVisibility (Variables|Default|GetSpiderHP) false false))

(event EventBeginPlay
  ;[1 1 1] BeginPlay Logic
  (|CallParentFunction)
  (bind _returnvalue (Actor|GetActorOfClass "/Game/NatsBlueprints/Blueprints/Player/BP_FirstPersonCharacter.BP_FirstPersonCharacter_C"))
  (Variables|Default|SetCharRef _returnvalue)
  (Utilities|Time|SetTimerbyEvent (delegate Custom|CheckIsChasing) 2.0 true)
  (Rendering|SetVisibility (Variables|Default|GetSpiderHP) false false))

(event EventTick
  (params (DeltaSeconds :type Float%20%28single-precision%29))
  ;[0 1 0.9818] PerTick
  (|CallParentFunction 0.0)
  (if (not (<= (Variables|Default|GetcurrHP) 0.0))
    ;;[1 1 1] PreventOverheal
    (if (>= (Variables|Default|GetcurrHP) (Variables|Default|GetmaxHP))
      (Variables|Default|SetcurrHP (Variables|Default|GetmaxHP)))
    ;;[1 1 1] HealthbarFaceCamera
    (Transformation|SetWorldRotation (Variables|Default|GetSpiderHP) (Math|Rotator|FindLookatRotation (Transformation|GetActorLocation) (.OutLocation (Actor|GetActorEyesViewPoint (Variables|Default|GetCharRef)))) false false)
    ;;[1 1 1] SetHealthbarPercent
    (CallFunction|UpdateHealthBar (Variables|Default|GetcurrHP))
    ;[0.0643 0.2771 1] prepare...
    (Utilities|FlowControl|Delay 0.1)
    (if (not (Variables|Default|GetisAttacking))
      ;[1 0.3015 0.0599] Point Blank
      (bind _outactors (Collision|SphereOverlapActors (Transformation|GetActorLocation) 1.4e+02 (Utilities|Array|MakeArray "ObjectTypeQuery3") 0))
      (bind _array_element (Utilities|Array|ForEachLoopwithBreak _outactors :!label _label)
        (:LoopBody
          (Utilities|Casting|CastToBP_FirstPersonCharacter _array_element)
          (Variables|Default|SetisAttacking true)
          (goto _label Break))
        (:Completed
          (if (Variables|Default|GetisAttacking)
            (Animation|Montage|PlayMontage (Variables|Character|GetMesh) "/Game/Assets/Animals/Spider/Spider_Attack_Montage.Spider_Attack_Montage"
              (:OnCompleted
                _)
              (:OnInterrupted
                _)
              (:OnNotifyBegin
                (bind _outactors_2 (Collision|SphereOverlapActors (Transformation|GetActorLocation) 1.6e+02 (Utilities|Array|MakeArray "ObjectTypeQuery3") 0))
                (bind _array_element_2 (Utilities|Array|ForEachLoopwithBreak _outactors_2 :!label _label_2)
                  (:LoopBody
                    (bind _asbp_first_person_character (Utilities|Casting|CastToBP_FirstPersonCharacter _array_element_2))
                    (Development|PrintString "OW")
                    (Default|OnHit _asbp_first_person_character 15.0)
                    (goto _label_2 Break)))))
            (Variables|Default|SetisAttacking false)))))))

(fn ConstructionScript)

(fn UpdateHealthBar
  (params (NewHP :type Float%20%28double-precision%29))
  (bind _asenemy_hp_widget (Utilities|Casting|CastToEnemyHP_Widget (UserInterface|GetUserWidgetObject (Variables|Default|GetSpiderHP))))
  (Default|SetHP _asenemy_hp_widget (/ NewHP (Variables|Default|GetmaxHP))))