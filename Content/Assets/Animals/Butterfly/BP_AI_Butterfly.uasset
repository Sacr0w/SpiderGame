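; Butterfly AI pawn that roams at random around the navmesh and destroys itself when its health runs out.
; RandomRoam picks a navigable point within a fixed radius, offsets it upward and calls AIMoveTo, restarting itself on success or failure.
; Tick polls CurrHP to handle death.
; BeginPlay caches the first-person character and starts roaming, while the pawn-sensing and chase events are empty.
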(event OnSeePawn(PawnSensing)
  (params (Pawn :type Pawn%20Object%20Reference)))

(event Custom|Random%20Roam
  (bind _randomlocation (Class|NavigationSystemV1|GetRandomLocationinNavigableRadius (Transformation|GetActorLocation) 1e+03 0 0))
  (AI|AIMoveTo self (Math|Vector|MakeVector (.x _randomlocation) (.y _randomlocation) (+ (.z _randomlocation) 1e+02)) 0 5.0 false
    (:OnSuccess
      _)
    (:OnFail
      _))
  (CallFunction|RandomRoam))

(event Custom|Chase%20Player)

(event EventBeginPlay
  (bind _returnvalue (Actor|GetActorOfClass "/Game/NatsBlueprints/Blueprints/BP_FirstPersonCharacter.BP_FirstPersonCharacter_C"))
  (Variables|Default|SetCharRef _returnvalue)
  (CallFunction|RandomRoam))

(event Collision|EventActorBeginOverlap
  (params (OtherActor :type Actor%20Object%20Reference)))

(event EventTick
  (params (DeltaSeconds :type Float%20%28single-precision%29))
  (if (<= (Variables|Default|GetcurrHP) 0.0)
    (Actor|DestroyActor)))

(fn ConstructionScript)